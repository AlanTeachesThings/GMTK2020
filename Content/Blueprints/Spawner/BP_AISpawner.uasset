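; AI spawner actor that spawns a set number of AI pawns at its location, either on BeginPlay or when the player comes within a radius.
; Proximity mode polls with a sphere trace on a looping timer, optionally requiring line of sight.
; A second timer spawns and counts each pawn, broadcasting per spawn and on completion.
; If reset is allowed, a completed spawner clears its count and re-initializes.
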(event Custom|Init%20Spawner
  (bind _spawner_type (Variables|Default|GetSpawner%20Type))
  ;[1 1 1] Execute appropriate spawner state
  (if (Utilities|Enum|Equal(Enum) _spawner_type "NewEnumerator1")
    (CallFunction|StartSpawner)
    (elif (Utilities|Enum|Equal(Enum) _spawner_type "NewEnumerator0")
      (Utilities|Time|SetTimerbyFunctionName 0 "ProximityCheck" 0.1 true))))

(event Custom|Start%20Spawner
  (if (== (Variables|Default|GetSpawn%20Counter) 0)
    (Utilities|FlowControl|Sequence
      (:then_0
        (Utilities|Time|ClearTimerbyFunctionName 0 "ProximityCheck") ; In proximity mode, we can stop checking proximity
      )
      (:then_1
        (CallFunction|SpawnWave (Variables|Default|GetAI%20type) (Variables|Default|GetTotal%20Number%20of%20AI%20to%20spawn) (Variables|Default|GetDelay%20Between%20Spawns))))
    (else
      (Development|PrintString "Expected Spawn Coutner to be 0"))))

(event EventBeginPlay
  (CallFunction|InitSpawner) ; We use a separate begin play event so we can call it again on restart (via Reset Spawner func)
)

(fn ConstructionScript
  (Rendering|Debug|DrawDebugSphere (Transformation|GetActorLocation) (Variables|Default|GetProximity%20Radius) 12 "(R=0.395026,G=0.970145,B=1.000000,A=1.000000)" 0.0 12.0))

(fn SpawnAI
  (params (AI%20Type :type BP%20Enemy%20Base%20Class%20Reference))
  ;[1 1 1] Spawn the actual object
  (bind _returnvalue (AI|SpawnAIFromClass AI%20Type 0 (Transformation|GetActorLocation) "0, 0, 0" true 0))
  (bind _asbp_enemy_base (Utilities|Casting|CastToBP_EnemyBase _returnvalue))
  (Default|CallOnAISpawned self _asbp_enemy_base)
  (return _asbp_enemy_base))

(fn SpawnWave
  (params (AI%20Type :type BP%20Enemy%20Base%20Class%20Reference) (Amount :type Integer) (TimeBetweenSpawns :type Float%20%28single-precision%29))
  (Variables|Default|SetAI%20type AI%20Type)
  (Variables|Default|SetIsAvailable false)
  (Variables|Default|SetTotal%20Number%20of%20AI%20to%20spawn Amount)
  (bind _returnvalue (Utilities|Time|SetTimerbyFunctionName 0 "SpawnAndCount" TimeBetweenSpawns true))
  (Variables|Default|SetSpawnTimerHandle _returnvalue))

(fn ResetSpawner
  (if (Variables|Default|GetAllow%20Spawner%20to%20be%20reset)
    (Utilities|Time|ClearandInvalidateTimerbyHandle (Variables|Default|GetSpawnTimerHandle))
    (Variables|Default|SetSpawn%20Counter 0)
    (Variables|Default|SetIsAvailable true)
    (CallFunction|InitSpawner)
    (return)
    (else
      (return))))

(fn ProximityCheck
  (bind _returnvalue (Transformation|GetActorLocation))
  (bind (_outhits _returnvalue_2) (Collision|MultiSphereTraceForObjects _returnvalue _returnvalue (Variables|Default|GetProximity%20Radius) (Utilities|Array|MakeArray "ObjectTypeQuery3") false 0 (select (Variables|Default|GetDraw%20Debug%20Proximity) "ForDuration" "None") true "(R=1.000000,G=0.000000,B=0.000000,A=1.000000)" "(R=0.000000,G=1.000000,B=0.000000,A=1.000000)" 0.1))
  (if _returnvalue_2
    (for _array_element _outhits
      (bind _asbp_player_char (Utilities|Casting|CastToBP_PlayerChar (.HitActor (Collision|BreakHitResult _array_element))))
      (if (Variables|Default|GetVisibility%20Check%20with%20Proximity) ; Optional line of sight check
        (|VisibilityTraceonconfirmedhitwithinradius _asbp_player_char)
        (else
          (CallFunction|StartSpawner))))))

(fn CountandCheckSpawnsComplete
  (bind _spawn_counter (Variables|Default|GetSpawn%20Counter))
  (Math|Integer|IncrementInt _spawn_counter
    (:%20%20
      (if (== _spawn_counter (Variables|Default|GetTotal%20Number%20of%20AI%20to%20spawn))
        (CallFunction|ResetSpawner)
        (Default|CallOnSpawnsComplete self)
        (Utilities|Time|PauseTimerbyHandle (Variables|Default|GetSpawnTimerHandle))))))

(fn SpawnandCount
  (CallFunction|SpawnAI (Variables|Default|GetAI%20type))
  (CallFunction|CountandCheckSpawnsComplete)
  (return))