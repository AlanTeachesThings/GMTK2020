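; BP_AIWaves runs a level's enemy waves, loading that level's rows from a data table when the GameMode's start-level event fires.
; Each wave goes to a random available spawner after a delay, then chains to the next immediately or once a spawner completes.
; Waves without a free spawner are counted as pending and retried on spawner completion.
; It tracks living enemies and broadcasts enemy deaths and completion of all waves.
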(event Custom|EnemySpawned
  (params (Spawner :type BP%20AI%20Spawner%20Object%20Reference) (Enemy :type BP%20Enemy%20Base%20Object%20Reference))
  ;[1 1 1] Bind to events to keep track of active enemies
  (EventDispatchers|BindEventtoOnDeath Enemy (delegate Custom|EnemyDeath))
  (Math|Integer|IncrementInt (Variables|LevelData|GetEnemyCount)))

(event Custom|SpawnWave
  (params (Spawner :type BP%20AI%20Spawner%20Object%20Reference) (WaveData :type AI%20Wave%20Structure) (Auto%20Spawn%20next%20wave :type Boolean))
  (bind (_level _aitype _amount _timebetweenspawns _startdelay _waitforwavecompletebeforenextwave) (Utilities|Struct|BreakAIWave WaveData))
  ;[1 1 1] Spawn wave on spawner using AIWave data. Can be called directly or run through SpawnNextWave in a level.
  (Utilities|FlowControl|Delay _startdelay)
  (Default|SpawnWave Spawner _aitype _amount _timebetweenspawns)
  (if Auto%20Spawn%20next%20wave
    (if _waitforwavecompletebeforenextwave
      (Variables|Default|SetWaitForWaveCompletedBeforeNextWave _waitforwavecompletebeforenextwave)
      (else
        (CallFunction|StartNextWave)))))

(event Custom|SpawnerComplete
  (params (Spawner :type BP%20AI%20Spawner%20Object%20Reference))
  (bind _numwavespending (Variables|Default|GetNumWavesPending))
  ;[1 1 1] Are there any pending waves that did not get available spawner? If not, are we waiting for wave complete before starting next?
  (if (> _numwavespending 0)
    (Math|Integer|DecrementInt _numwavespending
      (:%20%20
        (CallFunction|StartNextWave)))
    (elif (Variables|Default|GetWaitForWaveCompletedBeforeNextWave)
      (Variables|Default|SetWaitForWaveCompletedBeforeNextWave false)
      (Utilities|FlowControl|Delay 0.2) ; For single enemy waves a short delay is necessary
      (CallFunction|StartNextWave))))

(event Custom|EnemyDeath
  (params (Character :type BP%20Char%20Base%20Object%20Reference))
  ;[1 1 1] Bind to events to keep track of active enemies
  (Default|CallOnEnemyDeath Character)
  (Math|Integer|DecrementInt (Variables|LevelData|GetEnemyCount)
    (:%20%20
      ;;[1 1 1] Check whether this was last enemy
      (bind _wavescomplete (CallFunction|CheckWavesComplete))
      (if _wavescomplete
        (Default|CallOnWavesCompleted)
        (CallFunction|ResetWaveCount)))))

(event Custom|StartLevel
  (params (Level :type Integer) (DelayDuration :type Float%20%28single-precision%29))
  ;[1 1 1] Start Level. Can be bound to Gamemode
  (bind _result (CallFunction|GetLevelDatafromDatatable Level))
  (Variables|LevelData|SetCurrentLevelWaves _result)
  (CallFunction|StartNextWave))

(fn ConstructionScript)

(fn Initialize
  (params (WavesData :type Data%20Table%20Object%20Reference) (Spawners :type Array%20of%20BP%20AI%20Spawner%20Object%20References))
  (Variables|Default|SetWavesData WavesData)
  (Utilities|FlowControl|Sequence
    (:then_0
      ;[1 1 1] Set spawners and bind to Spawner events
      (bind _output_get (Variables|Default|SetAISpawners Spawners))
      (for _array_element _output_get
        (EventDispatchers|BindEventtoOnAISpawned _array_element (EventDispatchers|CreateEvent :!event Custom|EnemySpawned))
        (EventDispatchers|BindEventtoOnSpawnsComplete _array_element (EventDispatchers|CreateEvent :!event Custom|SpawnerComplete))))
    (:then_1
      ;[1 1 1] Bind to OnStartLevel
      (bind _asgm_base (Utilities|Casting|CastToGM_Base (Game|GetGameMode)))
      (EventDispatchers|BindEventtoOnStartLevel _asgm_base (EventDispatchers|CreateEvent :!event Custom|StartLevel)))))

(fn CheckWavesComplete
  (Utilities|FlowControl|Sequence
    (:then_0
      ;[1 1 1] Has last wave been activated?
      (if (not (>= (Variables|LevelData|GetCurrentWave) (Utilities|Array|Length (Variables|LevelData|GetCurrentLevelWaves)))) ; When True go to next check in sequence
        (return false)))
    (:then_1
      ;[1 1 1] Check if all spawners are done spawning
      (for _array_element (Variables|Default|GetAISpawners)
        (if (not (Variables|/Game/Blueprints/Spawner/BP_AISpawner.BP_AISpawner_C|GetIsAvailable _array_element))
          (return false))))
    (:then_2
      ;[1 1 1] Check if all enemies are dead
      (if (== (Variables|LevelData|GetEnemyCount) 0)
        (return true)
        (else
          (return false))))))

(fn GetLevelDatafromDatatable
  (params (Level :type Integer))
  (bind _outrownames (DataTable|GetDataTableRowNames (Variables|Default|GetWavesData)))
  (for _array_element _outrownames
    (bind _returnvalue (Utilities|GetDataTableRow (Variables|Default|GetWavesData) _array_element)
      (:then
        (if (== Level (.Level (Utilities|Struct|BreakAIWave _returnvalue)))
          (Utilities|Array|Add (LocalVariables|GettempAIWaves) _returnvalue)))))
  (return (LocalVariables|GettempAIWaves)))

(fn FindAvailableSpawner
  (bind _aispawners (Variables|Default|GetAISpawners))
  (Utilities|Array|Shuffle _aispawners)
  (for _array_element _aispawners
    (if (Variables|/Game/Blueprints/Spawner/BP_AISpawner.BP_AISpawner_C|GetIsAvailable _array_element)
      (return _array_element)))
  (return 0))

(fn StartNextWave
  (bind _currentlevelwaves (Variables|LevelData|GetCurrentLevelWaves))
  ;[1 1 1] Check if there are more waves available, find a spawner, and spawn it.
  (if (< (Variables|LevelData|GetCurrentWave) (Utilities|Array|Length _currentlevelwaves))
    (bind _aispawner (CallFunction|FindAvailableSpawner))
    (Utilities|IsValid _aispawner
      (:Is%20Valid
        (CallFunction|SpawnWave _aispawner (Utilities|Array|Get(acopy) _currentlevelwaves (Variables|LevelData|GetCurrentWave)) true)
        (Math|Integer|IncrementInt (Variables|LevelData|GetCurrentWave)))
      (:Is%20Not%20Valid
        (Math|Integer|IncrementInt (Variables|Default|GetNumWavesPending))))))

(fn ResetWaveCount
  (Variables|LevelData|SetCurrentWave 0))