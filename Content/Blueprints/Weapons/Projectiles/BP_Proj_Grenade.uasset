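; Grenade projectile Blueprint that lobs toward a target location and deals radial damage on hit.
; On BeginPlay, the Velocity variable serves as the destination, and SetDestination computes an arced launch with increased gravity via SuggestProjectileVelocityCustomArc.
; Tick draws a debug circle at the target as feed-forward, its size and thickness driven by remaining distance.
; Hit flashes the blast radius, applies damage, plays a sound and destroys the actor.
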(event EventBeginPlay
  (bind _velocity (Variables|Default|GetVelocity))
  (|CallParentFunction)
  (CallFunction|SetDestination _velocity 4.0 (Variables|Default|GetArch))
  (Variables|Default|SetInitial%20Distance (Math|Vector|Distance(Vector) _velocity (Transformation|GetActorLocation))))

(event EventTick
  (params (DeltaSeconds :type Float%20%28single-precision%29))
  (bind _returnvalue (Transformation|GetActorLocation))
  (bind _initial_distance (Variables|Default|GetInitial%20Distance))
  (bind _radius (Variables|Default|GetRadius))
  (bind _velocity (Variables|Default|GetVelocity))
  (bind _returnvalue_2 (Math|Vector|Distance(Vector) _velocity _returnvalue))
  (bind _returnvalue_3 (* _radius 2.0))
  (bind _returnvalue_4 (Math|Float|MapRangeClamped _returnvalue_2 _initial_distance 0.0 _returnvalue_3 _radius))
  ;[1 1 1] Visualize FeedForward
  (Rendering|Debug|DrawDebugCircle (Variables|Default|GetVelocity) _returnvalue_4 100 (Variables|Default|GetColor) 0.0 (Math|Float|Lerp 1.0 1e+01 (- 2.0 (/ _returnvalue_4 _radius))) "1.000000,0.000000,0.000000" "0.000000,1.000000,0.000000"))

(event Collision|EventHit
  (params (MyComp :type Primitive%20Component%20Object%20Reference) (Other :type Actor%20Object%20Reference) (OtherComp :type Primitive%20Component%20Object%20Reference) (bSelfMoved :type Boolean) (HitLocation :type Vector :default "0, 0, 0") (HitNormal :type Vector :default "0, 0, 0") (NormalImpulse :type Vector :default "0, 0, 0") (Hit :type Hit%20Result%20Structure%20%28by%20ref%29))
  ;[1 1 1] Hit Feedback
  (Rendering|Debug|DrawDebugCircle HitLocation (Variables|Default|GetRadius) 100 (Variables|Default|GetColor) 0.1 1e+01 "1.000000,0.000000,0.000000" "0.000000,1.000000,0.000000")
  (Game|Damage|ApplyRadialDamage (Variables|Default|GetDamage) HitLocation (Variables|Default|GetRadius) 0 (Utilities|Array|MakeArray self) (Components|GetOwner) (Game|GetInstigatorController) false "ECC_Visibility")
  (Audio|PlaySoundatLocation (Variables|Default|GetHit%20Sound) HitLocation "0, 0, 0" 1.0 1.0 0.0 "/Game/Assets/Audio/BaseAttenuation.BaseAttenuation" "/Game/Assets/Audio/BaseConcurrency.BaseConcurrency" 0)
  (Actor|DestroyActor))

(fn ConstructionScript
  (|CallParentFunction))

(fn SetDestination
  (params (Destination :type Vector) (ProjectileGravityScale :type Float%20%28single-precision%29) (ArcParam :type Float%20%28single-precision%29))
  (bind _projectilemovement (Variables|Default|GetProjectileMovement))
  (Variables|/Script/Engine.ProjectileMovementComponent|SetProjectileGravityScale _projectilemovement ProjectileGravityScale)
  (bind _outlaunchvelocity (Game|SuggestProjectileVelocityCustomArc (Transformation|GetActorLocation) Destination (Components|Movement|GetGravityZ _projectilemovement) ArcParam))
  (Variables|/Script/Engine.MovementComponent|SetVelocity _projectilemovement _outlaunchvelocity))