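; Heal grenade projectile Blueprint that extends a parent projectile with homing toward a HomingTarget.
; Shortly after BeginPlay, it sets the projectile movement's max speed, assigns HomingTarget as the homing component and prints that component's name for debugging.
; An empty Tick override suppresses the parent's destination visualization.
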(event EventBeginPlay
  (|CallParentFunction)
  (Utilities|FlowControl|Delay 0.1)
  (Variables|/Script/Engine.ProjectileMovementComponent|SetMaxSpeed (Variables|Default|GetProjectileMovement) 2.5e+03)
  (bind _output_get (Variables|/Script/Engine.ProjectileMovementComponent|SetHomingTargetComponent (Variables|Default|GetProjectileMovement) (Variables|Default|GetHoming%20Target)))
  (Development|PrintString (Utilities|GetDisplayName _output_get)))

(event EventTick
  (params (DeltaSeconds :type Float%20%28single-precision%29))
  ;[1 1 1] We ovveride this so we dont get the destination visualization
)

(fn ConstructionScript
  (|CallParentFunction))