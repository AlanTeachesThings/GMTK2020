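; BP_Proj_Progressive is a weapon projectile that grows and changes color over its lifetime, then destroys itself.
; On BeginPlay, the SizeLerp timeline has its play rate scaled by TimeBeforeExplosion, then interpolates from Size to MaxSize and from Color toward a pinkish red.
; The actor is destroyed when the timeline finishes.
; The construction script sets the PointLight to the starting Color.
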(event EventBeginPlay
  (bind _size_lerp (Variables|Default|GetSize%20Lerp))
  (bind _returnvalue (Components|Timeline|GetPlaybackPosition _size_lerp))
  (|CallParentFunction)
  (Components|Timeline|SetPlayRate _size_lerp (/ 1.0 (Variables|Default|GetTimeBeforeExplosion)))
  (Timeline|Size%20Lerp Play
    (:Update
      (CallFunction|SetSize (Math|Float|Lerp (Variables|Default|GetSize) (Variables|Default|GetMax%20Size) _returnvalue))
      (CallFunction|SetColor (Math|Color|Lerp(LinearColor) (Variables|Default|GetColor) "(R=1.000000,G=0.049568,B=0.199456,A=1.000000)" _returnvalue)))
    (:Finished
      (Actor|DestroyActor))))

(fn ConstructionScript
  (|CallParentFunction)
  (Rendering|Components|Light|SetLightColor (Variables|Default|GetPointLight) (Variables|Default|GetColor) true))