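; Burst rifle weapon Blueprint that fires a fixed number of projectiles per trigger press, with a cooldown between bursts.
; StartBurst fires immediately and starts a looping fire-rate timer, which the Fire event clears once the burst's projectile count is reached.
; It also blocks the player character's movement and rotation for the burst duration.
; A separate one-shot timer governs the reset that re-enables bursting.
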(event EventTriggerPressed
  (if (Variables|Default|GetCanBurst)
    (CallFunction|StartBurst)))

(event EventFire
  (|CallParentFunction)
  ;[1 1 1] Keep track of projectiles fired in burst and stop firing after.
  (bind _result (Math|Integer|IncrementInt (Variables|Default|GetNumProjFired))
    (:%20%20
      (if (>= _result (Variables|Default|GetNumProjInBurst))
        (Utilities|Time|ClearandInvalidateTimerbyHandle (Variables|Default|GetBurstTimerHandle))))))

(event EventBeginPlay
  (|CallParentFunction)
  (bind _asbp_player_char (Utilities|Casting|CastToBP_PlayerChar (Game|GetInstigator)))
  (Variables|Default|SetPlayerCharRef _asbp_player_char))

(fn ConstructionScript
  (|CallParentFunction))

(fn StartBurst
  (Default|SetCannotMoveTimer (Variables|Default|GetPlayerCharRef) (* (CallFunction|GetFireRate) (Math|Conversions|ToFloat(Integer) (Variables|Default|GetNumProjInBurst))))
  ;[1 1 1] Start Burst. Counting of proj is done in event graph.
  (Default|SetCannotRotateTimer (Variables|Default|GetPlayerCharRef) (* (CallFunction|GetFireRate) (Math|Conversions|ToFloat(Integer) (Variables|Default|GetNumProjInBurst))))
  (Variables|Default|SetCanBurst false)
  (CallFunction|Fire)
  (bind _returnvalue (Utilities|Time|SetTimerbyEvent (EventDispatchers|CreateEvent :!event Fire) (CallFunction|GetFireRate) true))
  (Variables|Default|SetBurstTimerHandle _returnvalue)
  ;[1 1 1] Reset Burst after timer
  (Utilities|Time|SetTimerbyEvent (EventDispatchers|CreateEvent :!event ResetBurst) (Variables|Default|GetTimeBetweenBursts)))

(fn ResetBurst
  (Variables|Default|SetCanBurst true)
  (Variables|Default|SetNumProjFired 0))