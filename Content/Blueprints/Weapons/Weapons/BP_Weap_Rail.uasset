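; Railgun weapon that charges while the trigger is held and fires on release past a minimum charge, or automatically at full charge.
; A timeline drives charge alpha, a decal progress indicator and the weapon color, then reverses five times faster to discharge.
; The SpawnProjectile override uses a multi sphere trace, scaling point damage and debug-line beam thickness by charge, and pushes physics bodies by damage.
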(event Custom|Reverse%20Charge
  (bind _decal_material (Variables|Runtime|GetDecal%20Material))
  ;[1 1 1] Charging Logic
  (Components|Timeline|SetPlayRate (Variables|Default|GetCharge) (/ 5.0 (Variables|ChargeWeapon|GetMaxChargeTime)))
  (bind (_direction _alpha) (Timeline|Charge Reverse)
    (:Update
      (bind _output_get (Variables|Runtime|SetCharge%20Alpha _alpha))
      (Rendering|Material|SetScalarParameterValue _decal_material "Progress" (Variables|Runtime|GetCharge%20Alpha) :!class /Script/Engine.MaterialInstanceDynamic)
      (Rendering|Material|SetVectorParameterValue _decal_material "Color" (Math|Color|Lerp(LinearColor) "(R=1.000000,G=0.868751,B=0.000000,A=1.000000)" "(R=1.000000,G=0.000000,B=0.353102,A=1.000000)" _output_get) :!class /Script/Engine.MaterialInstanceDynamic)
      (if (> (Variables|Runtime|GetCharge%20Alpha) (Variables|ChargeWeapon|GetMinCharge)) ; We do this for to instantly change color and give feedback to the player that they can shoot
        (Variables|Default|SetColor (Math|Color|Lerp(LinearColor) "(R=1.000000,G=0.868751,B=0.000000,A=1.000000)" "(R=1.000000,G=0.000000,B=0.353102,A=1.000000)" _output_get))
        (else
          (Variables|Default|SetColor (Variables|Runtime|GetDefault%20Color)))))
    (:Finished
      (switch Utilities|FlowControl|Switch|SwitchonETimelineDirection _direction
        (:Forward
          (CallFunction|Fire))))))

(event Custom|Start%20Charge
  (bind _decal_material (Variables|Runtime|GetDecal%20Material))
  ;[1 1 1] Charging Logic
  (Components|Timeline|SetPlayRate (Variables|Default|GetCharge) (/ 1.0 (Variables|ChargeWeapon|GetMaxChargeTime)))
  (bind (_direction _alpha) (Timeline|Charge PlayFromStart)
    (:Update
      (bind _output_get (Variables|Runtime|SetCharge%20Alpha _alpha))
      (Rendering|Material|SetScalarParameterValue _decal_material "Progress" (Variables|Runtime|GetCharge%20Alpha) :!class /Script/Engine.MaterialInstanceDynamic)
      (Rendering|Material|SetVectorParameterValue _decal_material "Color" (Math|Color|Lerp(LinearColor) "(R=1.000000,G=0.868751,B=0.000000,A=1.000000)" "(R=1.000000,G=0.000000,B=0.353102,A=1.000000)" _output_get) :!class /Script/Engine.MaterialInstanceDynamic)
      (if (> (Variables|Runtime|GetCharge%20Alpha) (Variables|ChargeWeapon|GetMinCharge)) ; We do this for to instantly change color and give feedback to the player that they can shoot
        (Variables|Default|SetColor (Math|Color|Lerp(LinearColor) "(R=1.000000,G=0.868751,B=0.000000,A=1.000000)" "(R=1.000000,G=0.000000,B=0.353102,A=1.000000)" _output_get))
        (else
          (Variables|Default|SetColor (Variables|Runtime|GetDefault%20Color)))))
    (:Finished
      (switch Utilities|FlowControl|Switch|SwitchonETimelineDirection _direction
        (:Forward
          (CallFunction|Fire))))))

(event EventBeginPlay
  ;[0.447 0.9701 1] Init
  (|CallParentFunction)
  (Variables|Runtime|SetDefault%20Color (Variables|Default|GetColor)))

(event EventFire
  (|CallParentFunction)
  (if (== (Variables|Runtime|GetCharge%20Alpha) 1.0)
    (CallFunction|ReverseCharge)))

(event EventSpawnProjectile
  (bind _spawntransform (CallFunction|CalculateProjSpawnTransform))
  (bind (_location _rotation) (Math|Transform|BreakTransform _spawntransform))
  ;[1 1 1] Trace Rail
  (bind _outhits (Collision|MultiSphereTraceForObjects _location (+ _location (* (Math|Vector|GetForwardVector _rotation) (Variables|ChargeWeapon|GetRailgun%20Range))) 2e+01 (Utilities|Array|MakeArray "ObjectTypeQuery1" "ObjectTypeQuery2" "ObjectTypeQuery4" "ObjectTypeQuery3") false (Utilities|Array|MakeArray (Components|GetOwner) self) "None"))
  (for _array_element _outhits
    (Variables|Runtime|SetHit _array_element)
    (Rendering|Debug|DrawDebugLine (.TraceStart (Collision|BreakHitResult _array_element)) (Math|Vector|SelectVector (.Location (Collision|BreakHitResult _array_element)) (.TraceEnd (Collision|BreakHitResult _array_element)) (.bBlockingHit (Collision|BreakHitResult _array_element))) "(R=1.000000,G=0.000000,B=0.068705,A=1.000000)" 3.0 (Math|Float|Lerp 1.0 1e+01 (Variables|Runtime|GetCharge%20Alpha)))
    ;[1 1 1] Apply Damage
    (bind _returnvalue (Game|Damage|ApplyPointDamage (.HitActor (Collision|BreakHitResult (Variables|Runtime|GetHit))) (Math|Float|Lerp (Variables|ChargeWeapon|GetMinDamage) (Variables|Default|GetDamage) (Variables|Runtime|GetCharge%20Alpha)) (Math|Vector|GetUnitDirection(Vector) (.TraceStart (Collision|BreakHitResult (Variables|Runtime|GetHit))) (.TraceEnd (Collision|BreakHitResult (Variables|Runtime|GetHit)))) (Variables|Runtime|GetHit) (Game|GetInstigatorController) self))
    ;[1 1 1] Phys Interaction TODO: Honestly should be a knockback component or something, that just reads dmg and converts it to impulses
    (if (Physics|IsSimulatingPhysics (.HitComponent (Collision|BreakHitResult (Variables|Runtime|GetHit))) "None")
      (Physics|AddImpulseatLocation (.HitComponent (Collision|BreakHitResult (Variables|Runtime|GetHit))) (* (.ImpactNormal (Collision|BreakHitResult (Variables|Runtime|GetHit))) (* _returnvalue -1.0 1e+03)) (.Location (Collision|BreakHitResult (Variables|Runtime|GetHit))) "None"))))

(event EventTriggerPressed
  ;[1 1 1] Trigger Logic
  (Variables|Default|SetTriggerIsPressed true)
  (CallFunction|StartCharge))

(event EventTriggerReleased
  ;[1 1 1] Trigger Logic
  (Variables|Default|SetTriggerIsPressed false)
  (if (> (Variables|Runtime|GetCharge%20Alpha) (Variables|ChargeWeapon|GetMinCharge))
    (Utilities|FlowControl|Sequence
      (:then_0
        (CallFunction|Fire))
      (:then_1
        (CallFunction|ReverseCharge :!label _label)))
    (else
      (goto _label))))

(fn ConstructionScript
  (|CallParentFunction)
  (bind _returnvalue (Rendering|Material|CreateDynamicMaterialInstance (Variables|Default|GetDecal) :!class /Script/Engine.DecalComponent))
  (bind _output_get (Variables|Runtime|SetDecal%20Material _returnvalue))
  (Rendering|Material|SetScalarParameterValue _output_get "Respawn Time" (Variables|ChargeWeapon|GetMaxChargeTime) :!class /Script/Engine.MaterialInstanceDynamic)
  (Rendering|Material|SetScalarParameterValue _output_get "Seconds Per Section" 0.0 :!class /Script/Engine.MaterialInstanceDynamic)
  (Rendering|Material|SetScalarParameterValue _output_get "Emissive" 1e+01 :!class /Script/Engine.MaterialInstanceDynamic))