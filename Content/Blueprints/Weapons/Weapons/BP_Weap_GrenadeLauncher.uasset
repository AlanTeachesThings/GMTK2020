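; BP_Weap_GrenadeLauncher is a grenade launcher weapon Blueprint that shows a debug targeting circle at the cursor's hit point.
; BeginPlay runs the parent logic, then caches the owning pawn as a BP_PlayerChar reference.
; Every Tick, cursor traces on the Visibility channel place the circle and write the hit location into Velocity.
; Tick has no active-weapon check; a TODO notes the missing callback.
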(event EventBeginPlay
  (|CallParentFunction)
  (bind _asbp_player_char (Utilities|Casting|CastToBP_PlayerChar (Variables|Default|GetPawn%20Ref)))
  (Variables|Default|SetPlayer%20Ref _asbp_player_char))

(event EventTick
  (params (DeltaSeconds :type Float%20%28single-precision%29))
  (bind _returnvalue (Game|GetPlayerController 0))
  (bind _hitresult (Game|Player|GetHitResultUnderCursorbyChannel _returnvalue "TraceTypeQuery1" true))
  (bind _location (Collision|BreakHitResult _hitresult))
  ;[1 1 1] TODO: Add proper callback when weapon is active
  (Rendering|Debug|DrawDebugCircle _location 1e+02 100 "(R=0.953125,G=0.262835,B=0.834243,A=1.000000)" 0.0 1e+01 "1.000000,0.000000,0.000000" "0.000000,1.000000,0.000000")
  (Variables|Default|SetVelocity _location))

(fn ConstructionScript
  (|CallParentFunction))