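; Progressive weapon, a child of a base weapon, whose accuracy and fire rate shift the longer the trigger is held.
; InputHold tracks press time through by-ref variables, and Fire uses it to lerp both stats from their BeginPlay defaults before resetting the timer and calling the parent.
; SpawnProjectile accepts only BP_Proj_Progressive, mapping hold time to its explosion delay and printing an error for other classes.
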(event EventTriggerReleased
  (|CallParentFunction)
  (Variables|Runtime|SetLast%20Input%20State false))

(event EventBeginPlay
  (|CallParentFunction)
  (Variables|Runtime|SetDefault%20Accuracy (Variables|Default|GetAccuracy))
  (Variables|Runtime|SetDefault%20Fire%20Rate (Variables|Default|GetFire%20Rate)))

(event EventFire
  (bind _last_input_state (Variables|Runtime|GetLast%20Input%20State))
  (bind _last_press_time (Variables|Runtime|GetLast%20Press%20Time))
  (bind _max_hold_time (Variables|Default|GetMax%20Hold%20Time))
  (bind _triggerispressed (Variables|Default|GetTriggerIsPressed))
  (bind _returnvalue (CallFunction|InputHold _triggerispressed _last_input_state _last_press_time))
  (bind _returnvalue_2 (Math|Float|NormalizetoRange _returnvalue 0.0 _max_hold_time))
  (bind _returnvalue_3 (Math|Float|Clamp(Float) _returnvalue_2))
  (Variables|Default|SetAccuracy (Math|Float|Lerp (Variables|Runtime|GetDefault%20Accuracy) (Variables|Default|GetMax%20Accuracy%20Charge) _returnvalue_3))
  (Variables|Default|SetFire%20Rate (Math|Float|Lerp (Variables|Runtime|GetDefault%20Fire%20Rate) (Variables|Default|GetMax%20Fire%20Rate%20Change) _returnvalue_3))
  (CallFunction|SetTimer (CallFunction|GetFireRate))
  (|CallParentFunction))

(fn ConstructionScript
  (|CallParentFunction))

(fn InputHold
  (params (Input :type Boolean) (Last%20Input%20State :type Boolean%20%28by%20ref%29) (Last%20Press%20Time :type Float%20%28single-precision%29%20%28by%20ref%29))
  (if (Math|Boolean|Equal(Boolean) Input Last%20Input%20State)
    _
    (else
      (|SetBy-RefVar Last%20Press%20Time (Utilities|Time|GetGameTimeinSeconds))
      (|SetBy-RefVar Last%20Input%20State Input)))
  (return (- (Utilities|Time|GetGameTimeinSeconds) Last%20Press%20Time)))

(fn SpawnProjectile
  (if (== (Variables|Default|GetProjectile) "/Game/Blueprints/Weapons/Projectiles/BP_Proj_Progressive.BP_Proj_Progressive_C")
    (Game|SpawnActorfromClass "/Game/Blueprints/Weapons/Projectiles/BP_Proj_Progressive.BP_Proj_Progressive_C" (CallFunction|CalculateProjSpawnTransform) "Undefined" self (Math|Float|MapRangeClamped (CallFunction|InputHold (Variables|Default|GetTriggerIsPressed) (Variables|Runtime|GetLast%20Input%20State) (Variables|Runtime|GetLast%20Press%20Time)) (Variables|Default|GetMax%20Hold%20Time) 0.0 0.3 1.0) false "1000.000000,0.000000,0.000000" (Variables|Default|GetDamage) 0 (Game|GetInstigator))
    (else
      (Development|PrintString "Progressive weapon requires progressive projectile"))))