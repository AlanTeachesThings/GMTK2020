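; Main menu player controller that lets each local player join, leave or start the game.
; It caches the GM_MainMenu game mode on BeginPlay and forwards menu input to it.
; Confirm requests activation by controller ID when the player has no pawn, or requests game start when a pawn is already possessed.
; Back asks the game mode to deactivate that controller ID.
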(event EventBeginPlay
  ;[1 1 1] Get Gamemode Ref
  (|CallParentFunction)
  (bind _asgm_main_menu (Utilities|Casting|CastToGM_MainMenu (Game|GetGameMode)))
  (Variables|Default|SetGameModeRef _asgm_main_menu))

(event Input|ActionEvents|InputActionMenuConfirm
  (params (Key :type Key%20Structure :default "None"))
  (bind _gamemoderef (Variables|Default|GetGameModeRef))
  (:Pressed
    ;[1 1 1] See if the player is already active
    (Utilities|IsValid (Pawn|GetControlledPawn self)
      (:Is%20Valid
        (Default|RequestStartGame _gamemoderef))
      (:Is%20Not%20Valid
        (Default|RequestActivate _gamemoderef (Class|GameplayStatics|GetPlayerControllerID self))))))

(event Input|ActionEvents|InputActionMenuBack
  (params (Key :type Key%20Structure :default "None"))
  (:Pressed
    (Default|Deactivate (Variables|Default|GetGameModeRef) (Class|GameplayStatics|GetPlayerControllerID self))))

(fn ConstructionScript
  (|CallParentFunction))