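; GM_PlainVanilla is a game mode that runs AI enemy waves and awards score for kills.
; On BeginPlay it gathers the level's AI spawners, warns if none exist, then spawns a BP_AIWaves actor initialized with the wave data and those spawners.
; It binds to that actor's enemy-death and waves-completed dispatchers.
; EnemyDeath adds score from a class-keyed EnemyScores map, printing a message for unlisted classes.
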(event EventBeginPlay
  (|CallParentFunction)
  (Utilities|FlowControl|Sequence
    (:then_0
      ;[1 1 1] Get all spawners in level
      (bind _outactors (Actor|GetAllActorsOfClass "/Game/Blueprints/Spawner/BP_AISpawner.BP_AISpawner_C"))
      (bind _output_get (Variables|Default|SetAISpawnersRef _outactors))
      (if (not (!= (Utilities|Array|Length _output_get) 0))
        (Development|PrintString "This Mode requires at least one AISpawner Object")))
    (:then_1
      ;[1 1 1] Spawn AI Waves Actor
      (bind _returnvalue (Game|SpawnActorfromClass "/Game/Blueprints/Spawner/BP_AIWaves.BP_AIWaves_C" (Math|Conversions|ToTransform(Vector) (Math|Vector|VectorZero)) "Undefined" 0 0))
      (Variables|Default|SetAIWavesRef _returnvalue)
      (Default|Initialize _returnvalue (Variables|Default|GetWavesData) (Variables|Default|GetAISpawnersRef))
      (EventDispatchers|BindEventtoOnEnemyDeath _returnvalue (EventDispatchers|CreateEvent :!event EnemyDeath))
      (EventDispatchers|BindEventtoOnWavesCompleted _returnvalue (EventDispatchers|CreateEvent :!event EndLevel)))))

(fn ConstructionScript
  (|CallParentFunction))

(fn EnemyDeath
  (params (Character :type BP%20Char%20Base%20Object%20Reference))
  (bind _returnvalue (Utilities|GetClass Character))
  (bind _enemyscores (Variables|Default|GetEnemyScores))
  (bind (_value _returnvalue_2) (Utilities|Map|Find _enemyscores _returnvalue))
  (if _returnvalue_2
    (CallFunction|AddScore _value)
    (else
      (Development|PrintString (Utilities|String|ToString(Text) (Utilities|Text|FormatText "Class {class} could not be found in EnemyScores" (Utilities|GetClassDisplayName _returnvalue)))))))