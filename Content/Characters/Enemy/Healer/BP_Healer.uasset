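; BP_Healer is an enemy character that fires healing grenades at other enemies.
; When an inventory item spawns, it runs the parent handler, then switches a grenade launcher weapon's projectile to the heal grenade.
; StartFire shuffles all BP_EnemyBase actors, takes the first as the weapon's homing target, and writes that actor's location into the weapon's Velocity before calling the parent fire logic.
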(event EventBndEvtInventoryK2NodeComponentBoundEvent0onInventoryItemSpawnedDelegateSignature
  (params (Spawned%20Actor :type Actor%20Object%20Reference))
  ;[1 1 1] yeah, this is buggy, its better to bind delegates to custom events then I guess, as then naming on children would be alright
  (|CallParentFunction Spawned%20Actor)
  (bind _asbp_weap_grenade_launcher (Utilities|Casting|CastToBP_Weap_GrenadeLauncher (Variables|Default|GetCurrent%20Weapon)))
  (Variables|/Game/Core/BP_WeaponBase.BP_WeaponBase_C|SetProjectile _asbp_weap_grenade_launcher "/Game/Blueprints/Weapons/Projectiles/BP_Proj_HealGranade.BP_Proj_HealGranade_C"))

(event EventStartFire
  (bind _current_weapon (Variables|Default|GetCurrent%20Weapon))
  (bind _outactors (Actor|GetAllActorsOfClass "/Game/Characters/Enemy/BP_EnemyBase.BP_EnemyBase_C"))
  (Utilities|Array|Shuffle _outactors)
  (Variables|/Game/Core/BP_WeaponBase.BP_WeaponBase_C|SetHoming%20Target _current_weapon (Variables|/Script/Engine.Actor|GetRootComponent (Utilities|Array|Get(acopy) _outactors)))
  (Variables|/Game/Core/BP_WeaponBase.BP_WeaponBase_C|SetVelocity _current_weapon (Transformation|GetActorLocation (Utilities|Array|Get(acopy) _outactors)))
  (|CallParentFunction))

(fn ConstructionScript
  (|CallParentFunction))