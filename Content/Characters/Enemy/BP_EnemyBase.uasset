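; BP_EnemyBase is the base enemy character, with a health bar, an inventory-spawned weapon with start/stop fire events, and AI control.
; On BeginPlay it sets up the health UI, starts its behaviour tree through BP_BaseAIController and sizes nav agent properties from the capsule.
; To keep crowds unstuck, capsule hits and overlaps launch it away from other enemies and record them briefly.
; Tick pushes it from their average location until a retriggerable delay clears the list.
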(event OnInventoryItemSpawned(Inventory)
  (params (Spawned%20Actor :type Actor%20Object%20Reference))
  (bind _asbp_weapon_base (Utilities|Casting|CastToBP_WeaponBase Spawned%20Actor))
  (Variables|Default|SetCurrent%20Weapon _asbp_weapon_base))

(event OnComponentHit(CapsuleComponent)
  (params (HitComponent :type Primitive%20Component%20Object%20Reference) (OtherActor :type Actor%20Object%20Reference) (OtherComp :type Primitive%20Component%20Object%20Reference) (NormalImpulse :type Vector :default "0, 0, 0") (Hit :type Hit%20Result%20Structure%20%28by%20ref%29))
  ;[1 1 1] Crowd management - tries to prevent AI from getting stuck within themselves
  (Utilities|RegisterNearbyEnemies OtherActor))

(event OnComponentBeginOverlap(CapsuleComponent)
  (params (OverlappedComponent :type Primitive%20Component%20Object%20Reference) (OtherActor :type Actor%20Object%20Reference) (OtherComp :type Primitive%20Component%20Object%20Reference) (OtherBodyIndex :type Integer) (bFromSweep :type Boolean) (SweepResult :type Hit%20Result%20Structure%20%28by%20ref%29))
  ;[1 1 1] Crowd management - tries to prevent AI from getting stuck within themselves
  (Utilities|RegisterNearbyEnemies OtherActor))

(event Custom|Start%20Fire
  (bind _current_weapon (Variables|Default|GetCurrent%20Weapon))
  (Utilities|IsValid _current_weapon
    (:Is%20Valid
      (Default|TriggerPressed _current_weapon))))

(event Custom|Stop%20Fire
  (bind _current_weapon (Variables|Default|GetCurrent%20Weapon))
  (Utilities|IsValid _current_weapon
    (:Is%20Valid
      (Default|TriggerReleased _current_weapon))))

(event EventBeginPlay
  ;[0 0.9708 1] Begin Play
  (|CallParentFunction)
  (Utilities|FlowControl|Sequence
    (:then_0
      (CallFunction|SetupHealthUI (UserInterface|GetUserWidgetObject (Variables|Default|GetHealthBar))))
    (:then_1
      (bind _asbp_base_aicontroller (Utilities|Casting|CastToBP_BaseAIController (AI|GetAIController (Pawn|GetController))))
      (Default|InitBehaviourTree _asbp_base_aicontroller (Variables|Default|GetBehaviour%20Tree) (Variables|Default|GetPlayer%20Object%20Key))
      (CallFunction|UpdateNavMovementVars))))

(event EventTick
  (params (DeltaSeconds :type Float%20%28single-precision%29))
  (|CallParentFunction DeltaSeconds)
  ;[1 1 1] Add a bit extra avoidance when enemies are stuck in each other
  (if (Utilities|Array|IsValidIndex (Variables|Runtime|GetEnemies%20near))
    (bind _returnvalue (Class|GameplayStatics|GetActorArrayAverageLocation (Variables|Runtime|GetEnemies%20near)))
    (Physics|AddForce (Variables|Character|GetCharacterMovement) (* (Math|Vector|GetUnitDirection(Vector) _returnvalue (Transformation|GetActorLocation)) 1e+05))))

(event EventOnDestroy
  (UserInterface|SetWidget (Variables|Default|GetHealthBar) 0) ; Remove Health Bar on death
  (|CallParentFunction))

(fn ConstructionScript
  (|CallParentFunction))

(fn UpdateNavMovementVars
  (bind _capsulecomponent (Variables|Default|GetCapsuleComponent))
  (bind (_outradius _outhalfheight) (Components|Capsule|GetScaledCapsuleSize _capsulecomponent))
  (Variables|/Script/Engine.NavMovementComponent|SetNavAgentProps (Variables|Character|GetCharacterMovement) (Utilities|Struct|MakeNavAgentProperties _outradius _outhalfheight -1.0 1.0 "None" false false true)))