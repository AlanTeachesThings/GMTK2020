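; Spline rail actor, filed under the Railer enemy, that carries registered actors along its optionally looping path.
; The construction script lays evenly spaced static meshes and spline mesh segments along the spline.
; Adding the first actor starts a timeline timed from spline length and speed; removing the last stops it.
; Each update staggers actors by a time delay, pushing distant ones along the rail and interpolating near ones to their target.
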(event Custom|Stop%20Movement
  (bind _time (Timeline|Spline%20Movement Stop)
    (:Update
      (CallFunction|MoveActorsAlongASpline _time (Variables|Default|GetTime%20Delay%20Between%20Parts) (Variables|Default|GetConstant%20Velocity)))))

(event Custom|Start%20Movement
  (params (Loop%20Time :type Float%20%28single-precision%29))
  (bind _spline_movement (Variables|Default|GetSpline%20Movement))
  (Components|Timeline|SetPlayRate _spline_movement (/ 1.0 Loop%20Time))
  (Class|TimelineComponent|SetFloatCurve _spline_movement (Variables|Default|GetMovement%20Float) "Time")
  (bind _time (Timeline|Spline%20Movement Play)
    (:Update
      (CallFunction|MoveActorsAlongASpline _time (Variables|Default|GetTime%20Delay%20Between%20Parts) (Variables|Default|GetConstant%20Velocity)))))

(event EventBeginPlay
  (Variables|Default|SetSpeed (/ (Spline|GetSplineLength (Variables|Default|GetSpline)) (Variables|Default|GetSpeed))))

(fn ConstructionScript
  (bind _spline (Variables|Default|GetSpline))
  (bind _spline_2 (Variables|Default|GetSpline))
  (bind _spline_3 (Variables|Default|GetSpline))
  (bind _returnvalue (Spline|GetSplineLength _spline_3))
  (bind _returnvalue_2 (/ _returnvalue 2e+02))
  (bind _returnvalue_3 (Math|Float|Truncate _returnvalue_2))
  (bind _returnvalue_4 (- _returnvalue_3 1))
  (Spline|SetClosedLoop (Variables|Default|GetSpline) (Variables|Default|GetLoop) true)
  (Utilities|FlowControl|Sequence
    (:then_0
      ;[1 1 1] Static Mesh Placement
      (if (> _returnvalue_3 0)
        (for _index (range 0 _returnvalue_4) ; Repeat loop for each mesh to add
          (bind _returnvalue_5 (AddComponent|AddStaticMeshComponent false (Math|Transform|MakeTransform (Spline|GetLocationatDistanceAlongSpline _spline_2 (* _index (/ (Spline|GetSplineLength (Variables|Default|GetSpline)) (Math|Conversions|ToFloat(Integer) _returnvalue_4))) "Local") (Spline|GetRotationatDistanceAlongSpline _spline_2 (* _index (/ (Spline|GetSplineLength (Variables|Default|GetSpline)) (Math|Conversions|ToFloat(Integer) _returnvalue_4))) "Local") "1,1,1"))) ; Add static mesh component
          (Transformation|AddRelativeRotation _returnvalue_5 (Math|Rotator|MakeRotator 9e+01 0.0 0.0) false false)
          (Transformation|AddWorldOffset _returnvalue_5 "0, 0,10.000000" false false))))
    (:then_1
      ;[1 1 1] Spline Mesh
      (for _index_2 (range 0 (- (Spline|GetNumberOfSplinePoints _spline) 1))
        (bind _returnvalue_6 (AddComponent|AddSplineMeshComponent false))
        (SplineMesh|SetStartandEnd _returnvalue_6 (.Location (Math|Transform|BreakTransform (Spline|GetTransformatSplinePoint _spline _index_2 "Local" false))) (* (* (Math|Vector|GetForwardVector (.Rotation (Math|Transform|BreakTransform (Spline|GetTransformatSplinePoint _spline _index_2 "Local" false)))) (.Scale (Math|Transform|BreakTransform (Spline|GetTransformatSplinePoint _spline _index_2 "Local" false)))) (Math|Vector|VectorLength (- (.Location (Math|Transform|BreakTransform (Spline|GetTransformatSplinePoint _spline _index_2 "Local" false))) (.Location (Math|Transform|BreakTransform (Spline|GetTransformatSplinePoint _spline (+ _index_2 1) "Local" false)))))) (.Location (Math|Transform|BreakTransform (Spline|GetTransformatSplinePoint _spline (+ _index_2 1) "Local" false))) (* (* (Math|Vector|GetForwardVector (.Rotation (Math|Transform|BreakTransform (Spline|GetTransformatSplinePoint _spline (+ _index_2 1) "Local" false)))) (.Scale (Math|Transform|BreakTransform (Spline|GetTransformatSplinePoint _spline (+ _index_2 1) "Local" false)))) (Math|Vector|VectorLength (- (.Location (Math|Transform|BreakTransform (Spline|GetTransformatSplinePoint _spline _index_2 "Local" false))) (.Location (Math|Transform|BreakTransform (Spline|GetTransformatSplinePoint _spline (+ _index_2 1) "Local" false)))))) true :!class /Script/Engine.SplineMeshComponent)))))

(fn MoveActorsAlongASpline
  (params (Time :type Float%20%28single-precision%29) (Delay :type Float%20%28single-precision%29) (Constant%20Velocity :type Boolean))
  (bind _spline (Variables|Default|GetSpline))
  (bind _spline_2 (Variables|Default|GetSpline))
  (for (_array_element _array_index) (Variables|Default|GetActors%20to%20Move)
    (LocalVariables|SetRoot%20Comp (Variables|/Script/Engine.Actor|GetRootComponent _array_element))
    (if (> (Math|Vector|Distance(Vector) (Transformation|GetWorldLocation (LocalVariables|GetRoot%20Comp)) (Spline|GetLocationatTime _spline_2 (Math|Float|SelectFloat (- Time (* _array_index Delay)) (- 1.0 (Math|Float|Absolute(Float) (- Time (* _array_index Delay)))) (>= (- Time (* _array_index Delay)) 0.0)) "World" Constant%20Velocity)) 2e+02)
      (Transformation|SetWorldLocationAndRotation (LocalVariables|GetRoot%20Comp) (Math|Vector|MakeVector (.x (+ (* (Spline|FindDirectionClosesttoWorldLocation _spline (Transformation|GetWorldLocation (LocalVariables|GetRoot%20Comp)) "World") (* (Utilities|Time|GetWorldDeltaSeconds) (+ (Math|Vector|Distance(Vector) (Transformation|GetWorldLocation (LocalVariables|GetRoot%20Comp)) (Spline|GetLocationatTime _spline_2 (Math|Float|SelectFloat (- Time (* _array_index Delay)) (- 1.0 (Math|Float|Absolute(Float) (- Time (* _array_index Delay)))) (>= (- Time (* _array_index Delay)) 0.0)) "World" Constant%20Velocity)) (Variables|Default|GetSpeed)))) (Spline|FindLocationClosesttoWorldLocation _spline (Transformation|GetWorldLocation (LocalVariables|GetRoot%20Comp)) "World"))) (.y (+ (* (Spline|FindDirectionClosesttoWorldLocation _spline (Transformation|GetWorldLocation (LocalVariables|GetRoot%20Comp)) "World") (* (Utilities|Time|GetWorldDeltaSeconds) (+ (Math|Vector|Distance(Vector) (Transformation|GetWorldLocation (LocalVariables|GetRoot%20Comp)) (Spline|GetLocationatTime _spline_2 (Math|Float|SelectFloat (- Time (* _array_index Delay)) (- 1.0 (Math|Float|Absolute(Float) (- Time (* _array_index Delay)))) (>= (- Time (* _array_index Delay)) 0.0)) "World" Constant%20Velocity)) (Variables|Default|GetSpeed)))) (Spline|FindLocationClosesttoWorldLocation _spline (Transformation|GetWorldLocation (LocalVariables|GetRoot%20Comp)) "World"))) (.z (Transformation|GetWorldLocation (LocalVariables|GetRoot%20Comp)))) (Class|SplineComponent|GetRotationatTime _spline_2 (Math|Float|SelectFloat (- Time (* _array_index Delay)) (- 1.0 (Math|Float|Absolute(Float) (- Time (* _array_index Delay)))) (>= (- Time (* _array_index Delay)) 0.0)) "World" Constant%20Velocity) false false)
      (else
        (Transformation|SetWorldLocationAndRotation (LocalVariables|GetRoot%20Comp) (Math|Interpolation|VInterpTo (Transformation|GetWorldLocation (LocalVariables|GetRoot%20Comp)) (Spline|GetLocationatTime _spline_2 (Math|Float|SelectFloat (- Time (* _array_index Delay)) (- 1.0 (Math|Float|Absolute(Float) (- Time (* _array_index Delay)))) (>= (- Time (* _array_index Delay)) 0.0)) "World" Constant%20Velocity) (Utilities|Time|GetWorldDeltaSeconds) (Variables|Default|GetInterpolation%20Speed)) (Class|SplineComponent|GetRotationatTime _spline_2 (Math|Float|SelectFloat (- Time (* _array_index Delay)) (- 1.0 (Math|Float|Absolute(Float) (- Time (* _array_index Delay)))) (>= (- Time (* _array_index Delay)) 0.0)) "World" Constant%20Velocity) false false)))))

(fn FindTimeClosesttoWorldLocation
  (params (Actor :type Actor%20Object%20Reference))
  (bind _spline (Variables|Default|GetSpline))
  (return (/ (Spline|GetDistanceAlongSplineatSplinePoint _spline (Math|Float|Truncate (Class|SplineComponent|FindInputKeyClosesttoWorldLocation (Variables|Default|GetSpline) (Spline|FindLocationClosesttoWorldLocation (Variables|Default|GetSpline) (Transformation|GetActorLocation Actor) "Local")))) (Spline|GetSplineLength _spline))))

(fn AddActor
  (params (Actor :type Actor%20Object%20Reference%20%28by%20ref%29))
  (bind _actors_to_move (Variables|Default|GetActors%20to%20Move))
  (Utilities|Array|Add _actors_to_move Actor)
  (if (== (Utilities|Array|Length _actors_to_move) 1)
    (CallFunction|StartMovement (Variables|Default|GetSpeed))))

(fn RemoveActor
  (params (Actor :type Actor%20Object%20Reference%20%28by%20ref%29))
  (bind _actors_to_move (Variables|Default|GetActors%20to%20Move))
  (Utilities|Array|RemoveItem _actors_to_move Actor)
  (if (== (Utilities|Array|Length _actors_to_move) 0)
    (CallFunction|StopMovement)))