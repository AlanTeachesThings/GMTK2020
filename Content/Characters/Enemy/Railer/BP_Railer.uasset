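; Railer enemy Blueprint that seeks out a rail and attaches itself to it.
; On BeginPlay it runs the EQS_Rails query for a single result, then AI-moves to that location when the query finishes.
; Move success and failure both add it to CurrentRail, which is not assigned here, and destruction removes it.
; FindRailFromClosestLocation is an unfinished stub with an empty loop over PotentialRails.
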(event Custom|Rail%20Search
  (params (QueryInstance :type Env%20Query%20Instance%20Blueprint%20Wrapper%20Object%20Reference) (QueryStatus :type EEnvQueryStatus%20Enum :default "Processing"))
  (bind _resultlocations (AI|EQS|GetQueryResultsasLocations QueryInstance))
  (AI|AIMoveTo self (Utilities|Array|Get(acopy) _resultlocations) 0 5e+01 false
    (:OnSuccess
      _)
    (:OnFail
      _))
  (Default|AddActor (Variables|Default|GetCurrent%20Rail) self))

(event EventBeginPlay
  (|CallParentFunction)
  (bind _returnvalue (AI|EQS|RunEQSQuery "/Game/Characters/Enemy/AI/EQS/EQS_Rails.EQS_Rails" self "SingleResult" "/Script/AIModule.EnvQueryInstanceBlueprintWrapper"))
  (EventDispatchers|BindEventtoOnQueryFinishedEvent _returnvalue (EventDispatchers|CreateEvent :!event Custom|Rail%20Search)))

(event EventOnDestroy
  (Default|RemoveActor (Variables|Default|GetCurrent%20Rail) self)
  (|CallParentFunction))

(fn ConstructionScript
  (|CallParentFunction))

(fn FindRailfromClosestLocation
  (params (TargetArray :type Vector%20%28by%20ref%29))
  (for _array_element (Variables|Default|GetPotential%20Rails)
    _))