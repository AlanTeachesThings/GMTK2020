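; BP_Grenadier is an enemy character that aims a grenade launcher at players.
; On StartFire it writes a target location into the current weapon's Velocity field, which the launcher reads as a location, then calls the parent fire logic.
; The target adds a player pawn's location to a velocity as a simple lead, but each comes from a separate random pick from GM_Base's PlayerPawns.
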(event EventStartFire
  (bind _asgm_base (Utilities|Casting|CastToGM_Base (Game|GetGameMode)))
  (Variables|/Game/Core/BP_WeaponBase.BP_WeaponBase_C|SetVelocity (Variables|Default|GetCurrent%20Weapon) (+ (Transformation|GetActorLocation (Utilities|GetArrayRandomElement (Variables|/Game/Core/GameMode/GM_Base.GM_Base_C|GetPlayer%20Pawns _asgm_base))) (Transformation|GetVelocity (Utilities|GetArrayRandomElement (Variables|/Game/Core/GameMode/GM_Base.GM_Base_C|GetPlayer%20Pawns _asgm_base))))) ; The GrenadeLauncher expects this to be a location
  (|CallParentFunction))

(fn ConstructionScript
  (|CallParentFunction))