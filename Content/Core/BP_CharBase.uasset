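; Base character Blueprint providing shared health feedback, knockback, aim-facing mesh rotation and death handling.
; Construction creates dynamic materials for body and indicator colors, while Tick interpolates the mesh toward AimDirection.
; Point and radial damage optionally launch the character by damage amount; health changes drive a timed green/red material shake.
; Destruction disables capsule collision, signals death and plays a scale timeline before destroying the actor; children can initialize a health bar.
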(event Custom|Health%20Modified
  (params (NewHealth :type Float%20%28single-precision%29) (Health%20Added :type Boolean))
  ;[1 1 1] Hit Feedback
  (CallFunction|HitShake 0.1 Health%20Added)
  (Utilities|FlowControl|RetriggerableDelay 0.1)
  (CallFunction|HitShake -0.1 Health%20Added) ; This is how we restore the original state (check MF_HitShake)
)

(event EventTick
  (params (DeltaSeconds :type Float%20%28single-precision%29))
  ;[1 0.9261 0.3375] Tick
  (CallFunction|RotateMeshTowardsAim (Variables|Character|GetInterp%20Mesh%20Rotation%20Speed)) ; Overidable
)

(event EventOnDestroy
  (Collision|SetCollisionEnabled (Variables|Collision|GetCapsuleComponent) "NoCollision")
  (Default|CallOnDeath self)
  (Variables|Runtime|SetDead false)
  (bind _scale (Timeline|DestroyScale Play) ; TODO:Replace with shader version
    (:Update
      (Transformation|SetActorScale3D (Math|Conversions|ToVector(Float) _scale)))
    (:Finished
      (Actor|DestroyActor))))

(event EventBeginPlay
  ;[0.2396 1 1] Begin Play
  (EventDispatchers|BindEventtoOnHealthChanged (Variables|Default|GetHealthComponent) (EventDispatchers|CreateEvent :!event Custom|Health%20Modified)))

(event Game|Damage|EventPointDamage
  (params (Damage :type Float%20%28single-precision%29) (DamageType :type Damage%20Type%20Object%20Reference) (HitLocation :type Vector :default "0, 0, 0") (HitNormal :type Vector :default "0, 0, 0") (HitComponent :type Primitive%20Component%20Object%20Reference) (BoneName :type Name :default "None") (ShotFromDirection :type Vector :default "0, 0, 0") (InstigatedBy :type Controller%20Object%20Reference) (DamageCauser :type Actor%20Object%20Reference) (HitInfo :type Hit%20Result%20Structure%20%28by%20ref%29))
  ;[1 1 1] Apply Knockback for both types of damage
  (if (Variables|Gameplay|GetRecieve%20Point%20DMG%20knockback)
    (Character|LaunchCharacter (* ShotFromDirection (Math|Float|MapRangeClamped Damage 0.0 1e+02 (Variables|Gameplay|GetMin%20knockback%20force) 2e+03)) false false)))

(event Game|Damage|EventRadialDamage
  (params (DamageReceived :type Float%20%28single-precision%29) (DamageType :type Damage%20Type%20Object%20Reference) (Origin :type Vector :default "0, 0, 0") (HitInfo :type Hit%20Result%20Structure%20%28by%20ref%29) (InstigatedBy :type Controller%20Object%20Reference) (DamageCauser :type Actor%20Object%20Reference))
  ;[1 1 1] Apply Knockback for both types of damage
  (if (Variables|Gameplay|GetRecieve%20Radial%20DMG%20knockback)
    (Character|LaunchCharacter (* (Math|Vector|GetUnitDirection(Vector) Origin (Transformation|GetActorLocation)) (Math|Float|MapRangeClamped DamageReceived 0.0 1e+02 (Variables|Gameplay|GetMin%20knockback%20force) 3e+03)) false false)))

(fn ConstructionScript
  (bind _mesh (Variables|Character|GetMesh))
  (Utilities|FlowControl|Sequence
    (:then_0
      (bind _mid (CallFunction|CreateMID _mesh))
      (Rendering|Material|SetVectorParameterValue _mid "Side Color" (Variables|Color|GetBody%20Side%20Color) :!class /Script/Engine.MaterialInstanceDynamic)
      (Rendering|Material|SetVectorParameterValue _mid "Top Color" (Variables|Color|GetBody%20Top%20Color) :!class /Script/Engine.MaterialInstanceDynamic))
    (:then_1
      (bind _mid_2 (CallFunction|CreateMID _mesh 1))
      (Rendering|Material|SetVectorParameterValue _mid_2 "Side Color" (Variables|Color|GetIndicator%20Side%20Color) :!class /Script/Engine.MaterialInstanceDynamic)
      (Rendering|Material|SetVectorParameterValue _mid_2 "Top Color" (Variables|Color|GetIndicator%20Top%20Color) :!class /Script/Engine.MaterialInstanceDynamic))))

(fn SetupHealthUI
  (params (WBP_HealthBar :type Object%20Object%20Reference))
  (bind _aswbp_health_bar (Utilities|Casting|CastToWBP_HealthBar WBP_HealthBar))
  (Default|InitialSetup _aswbp_health_bar (Variables|Default|GetHealthComponent))
  (return))

(fn RotateMeshTowardsAim
  (params (InterpSpeed :type Float%20%28single-precision%29))
  (bind _mesh (Variables|Character|GetMesh))
  (Transformation|SetWorldRotation _mesh (Math|Interpolation|RInterpTo (Transformation|GetWorldRotation _mesh) (Math|Conversions|RotationFromXVector (Variables|Runtime|GetAimDirection)) (Utilities|Time|GetWorldDeltaSeconds) InterpSpeed) false false)
  (return))

(fn HitShake
  (params (Effect%20Duration :type Float%20%28single-precision%29) (Heal? :type Boolean))
  (bind _mesh (Variables|Character|GetMesh))
  (Rendering|Material|SetScalarParameterValueonMaterials _mesh "Start Time" (Utilities|Time|GetGameTimeinSeconds))
  (Rendering|Material|SetScalarParameterValueonMaterials _mesh "Duration" Effect%20Duration)
  (Rendering|Material|SetVectorParameterValueonMaterials _mesh "HitColor" (Math|Conversions|ToVector(LinearColor) (Math|Color|SelectColor "(R=0.000000,G=1.000000,B=0.098716,A=1.000000)" "(R=1.000000,G=0.000000,B=0.121763,A=1.000000)" Heal?))))