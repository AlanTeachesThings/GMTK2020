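; BP_DoubleTap is a pickup that applies a temporary fire rate multiplier to the weapons of whoever picks it up.
; On pickup, it loops over the owner's Inventory runtime objects, calls UpdateFireRate on each BP_WeaponBase and records it in WeaponsAffected.
; On expiry, it sets those recorded weapons back to a 1.0 multiplier, so only weapons held at pickup time are affected.
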(event EventOnExpired
  (for _array_element (Variables|Default|GetWeapons%20Affected)
    (Default|UpdateFireRate _array_element 1.0)))

(event EventOnPickedUp
  (params (Owner :type Actor%20Object%20Reference))
  (for _array_element (Variables|/Game/Core/Components/Inventory.Inventory_C|GetInventory%20Runtime%20Object (Actor|GetComponentbyClass Owner "/Game/Core/Components/Inventory.Inventory_C"))
    (bind _asbp_weapon_base (Utilities|Casting|CastToBP_WeaponBase _array_element))
    (Default|UpdateFireRate _asbp_weapon_base (Variables|Default|GetFire%20Rate%20Multiplier))
    (Utilities|Array|Add (Variables|Default|GetWeapons%20Affected) _asbp_weapon_base)))

(fn ConstructionScript
  (|CallParentFunction))