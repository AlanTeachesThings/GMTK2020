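; Base projectile actor that flies forward, optionally homing, and deals point damage on hit before destroying itself.
; Construction applies color and size; BeginPlay adds the instigator's speed to launch velocity, ignores its collision and sets whether projectiles collide with each other.
; Hits push physics objects and play a sound on Pawns, while Tick draws a debug-line trail.
; The projectile-on-projectile explosion is deliberately disconnected.
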(event EventBeginPlay
  (Game|Components|ProjectileMovement|SetVelocityinLocalSpace (Variables|Default|GetProjectileMovement) (Math|Vector|MakeVector (+ (.x (Variables|Default|GetVelocity)) (CallFunction|VelocityInheritance)) 0.0 0.0))
  (CallFunction|IgnoreCollisionwithOwner)
  (Audio|PlaySoundatLocation (Variables|Default|GetFired%20Sound) (Transformation|GetActorLocation) "0, 0, 0" 1.0 1.0 0.0 "/Game/Assets/Audio/BaseAttenuation.BaseAttenuation" "/Game/Assets/Audio/BaseConcurrency.BaseConcurrency" 0)
  (CallFunction|SetResponsetoOtherProjectiles (Variables|Default|GetCollide%20with%20other%20projectiles))
  (Variables|/Script/Engine.ProjectileMovementComponent|SetHomingTargetComponent (Variables|Default|GetProjectileMovement) (Variables|Default|GetHoming%20Target))
  (Variables|Default|SetInstigator%20Controller (Game|GetInstigatorController)))

(event EventTick
  (params (DeltaSeconds :type Float%20%28single-precision%29))
  (CallFunction|RenderTrail 0.2))

(event Collision|EventHit
  (params (MyComp :type Primitive%20Component%20Object%20Reference) (Other :type Actor%20Object%20Reference) (OtherComp :type Primitive%20Component%20Object%20Reference) (bSelfMoved :type Boolean) (HitLocation :type Vector :default "0, 0, 0") (HitNormal :type Vector :default "0, 0, 0") (NormalImpulse :type Vector :default "0, 0, 0") (Hit :type Hit%20Result%20Structure%20%28by%20ref%29))
  (bind _output_get (Variables|Default|SetHit%20Result Hit))
  (|ApplyInpulsetoPhysObjects)
  (|SpawnEmitterifhitanotherprojectile)
  (Utilities|Casting|CastToPawn Other
    (:then
      (Audio|PlaySoundatLocation (Variables|Default|GetHit%20Sound) (.Location (Collision|BreakHitResult _output_get)) "0, 0, 0" 1.0 1.0 0.0 "/Game/Assets/Audio/BaseAttenuation.BaseAttenuation" "/Game/Assets/Audio/BaseConcurrency.BaseConcurrency" 0))
    (:CastFailed
      _))
  (Game|Damage|ApplyPointDamage Other (Variables|Default|GetDamage) (Math|Vector|GetUnitDirection(Vector) (Transformation|GetActorLocation) (.Location (Collision|BreakHitResult _output_get))) (Variables|Default|GetHit%20Result) (Variables|Default|GetInstigator%20Controller) self)
  (Actor|DestroyActor))

(fn ConstructionScript
  (CallFunction|SetColor (Variables|Default|GetColor))
  (CallFunction|SetSize (Variables|Default|GetSize)))

(fn SetResponsetoOtherProjectiles
  (params (ShouldBlock :type Boolean))
  (Collision|SetCollisionResponsetoChannel (Variables|Default|GetProjectileMesh) "ECC_GameTraceChannel1" (select ShouldBlock "ECR_Block" "ECR_Ignore"))
  (return))

(fn IgnoreCollisionwithOwner
  (bind _asprimitive_component (Utilities|Casting|CastToPrimitiveComponent (Variables|/Script/Engine.Actor|GetRootComponent (Game|GetInstigator))))
  (Collision|IgnoreActorwhenMoving _asprimitive_component self true) ; Tell our instigator to ignore this projectile
  (Collision|IgnoreActorwhenMoving (Variables|Default|GetProjectileMesh) (Game|GetInstigator) true) ; Tell this projectile to ignore the instigating character
)

(fn SetSize
  (params (Size :type Float%20%28single-precision%29))
  (Transformation|SetWorldScale3D (Variables|Default|GetProjectileMesh) (Math|Conversions|ToVector(Float) (/ Size 25.0))))

(fn SetColor
  (params (InLinearColor :type Linear%20Color%20Structure))
  (Rendering|Material|SetVectorParameterValueonMaterials (Variables|Default|GetProjectileMesh) "Color" (Math|Conversions|ToVector(LinearColor) InLinearColor)))

(fn RenderTrail
  (params (Duration :type Float%20%28single-precision%29))
  (bind _returnvalue (Transformation|GetActorLocation))
  (Rendering|Debug|DrawDebugLine (Math|Vector|SelectVector (Transformation|GetActorLocation) (Variables|Runtime|GetLast%20Pos) (Math|Vector|Equal(Vector) (Variables|Runtime|GetLast%20Pos) "0, 0, 0" 0.0001)) _returnvalue "(R=0.781250,G=0.755802,B=0.000000,A=1.000000)" Duration 2.0)
  (Variables|Runtime|SetLast%20Pos _returnvalue))

(fn VelocityInheritance
  (return (Math|Vector|VectorLength (Transformation|GetVelocity (Game|GetInstigator)))))