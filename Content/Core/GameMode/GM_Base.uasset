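; GM_Base is the base game mode that runs the five-level game flow: level start and end, score, game over, completion and pause.
; On BeginPlay it caches GameState, HUD and GameInstance, then opens a menu screen for GM_MainMenu, or opens the HUD and starts the level after a short delay.
; GameInstance tracks level progress and gates pawn spawning to active players; GameState holds score, and dispatchers broadcast gameplay events.
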(event EventBeginPlay
  (Utilities|FlowControl|Sequence
    (:then_0
      ;[1 1 1] Get GameState reference
      (bind _asgs_base (Utilities|Casting|CastToGS_Base (Game|GetGameState)))
      (Variables|Default|SetGameStateRef _asgs_base))
    (:then_1
      ;[1 1 1] Get HUD reference
      (bind _asbp_hud_base (Utilities|Casting|CastToBP_HudBase (HUD|GetHUD (Game|GetPlayerController 0))))
      (Variables|Default|SetHUDref _asbp_hud_base))
    (:then_2
      ;[1 1 1] Get Game Instance reference
      (bind _asgi_base (Utilities|Casting|CastToGI_Base (Game|GetGameInstance)))
      (Variables|Default|SetGameInstanceRef _asgi_base))
    (:then_3
      ;[1 1 1] Open MainMenu. If we're not in MainMenu, Start Level after giving all objects time to BeginPlay
      (Utilities|Casting|CastToGM_MainMenu self
        (:then
          (bind _asgi_base_2 (Utilities|Casting|CastToGI_Base (Game|GetGameInstance)))
          (CallFunction|OpenScreen 0 (Variables|/Game/Core/GameMode/GI_Base.GI_Base_C|GetScreenToOpen _asgi_base_2)))
        (:CastFailed
          (Utilities|FlowControl|Delay 0.2)
          (Default|OpenHUD (Variables|Default|GetHUDref))
          (CallFunction|StartNextLevel))))))

(event EventInitStartSpot
  (params (StartSpot :type Actor%20Object%20Reference) (NewPlayer :type Controller%20Object%20Reference))
  ;[1 1 1] Set Starting Spot player TODO: Should this be adapted for multiplayer?
  (|CallParentFunction StartSpot NewPlayer)
  (bind _asbp_char_base (Utilities|Casting|CastToBP_CharBase (Pawn|GetControlledPawn NewPlayer)))
  (Utilities|Array|AddUnique (Variables|Default|GetPlayer%20Pawns) _asbp_char_base))

(event Custom|StartNextLevel
  (bind _newlevel (CallFunction|IncrementLevel))
  (Default|CallOnStartLevel _newlevel (Variables|Default|GetDelayBeforeStartLevel)))

(event Custom|EndLevel
  (bind _delayafterendlevel (Variables|Default|GetDelayAfterEndLevel))
  (bind _asgi_base (Utilities|Casting|CastToGI_Base (Game|GetGameInstance)))
  (if (== (Variables|/Game/Core/GameMode/GI_Base.GI_Base_C|GetCurrentLevel _asgi_base) 5)
    (CallFunction|GameComplete)
    (else
      (Default|CallOnEndLevel (Variables|/Game/Core/GameMode/GI_Base.GI_Base_C|GetCurrentLevel _asgi_base) _delayafterendlevel) ; Only gets called on levels 1-4
      (Utilities|FlowControl|Delay _delayafterendlevel)
      (bind _asgi_base_2 (Utilities|Casting|CastToGI_Base (Game|GetGameInstance)))
      (Game|OpenLevel(byName) (Utilities|Array|Get(acopy) (Variables|Default|GetLevelNames) (Variables|/Game/Core/GameMode/GI_Base.GI_Base_C|GetCurrentLevel _asgi_base_2))))))

(event Custom|GameOver
  (Default|CallOnGameOver (Variables|/Game/Core/GameMode/GS_Base.GS_Base_C|GetScore (Variables|Default|GetGameStateRef))))

(event Custom|AddScore
  (params (Amount :type Integer))
  (bind _total (Default|AddScore (Variables|Default|GetGameStateRef) Amount))
  (Default|CallOnScoreAdded Amount _total))

(event Custom|Reset
  (Default|Reset (Variables|Default|GetGameStateRef)))

(event Custom|GameComplete
  (Default|CallOnGameComplete (Variables|/Game/Core/GameMode/GS_Base.GS_Base_C|GetScore (Variables|Default|GetGameStateRef))))

(event Custom|TogglePause
  (Utilities|Casting|CastToGM_MainMenu self ; Check that we are not in Main Menu
    (:CastFailed
      (Utilities|FlowControl|FlipFlop
        (:A
          (Game|SetGamePaused true)
          (CallFunction|OpenScreen 0 "/Game/UI/MenuScreens/WBP_PauseScreen.WBP_PauseScreen_C"))
        (:B
          (Game|SetGamePaused false))))))

(fn ConstructionScript)

(fn IncrementLevel
  (bind _gameinstanceref (Variables|Default|GetGameInstanceRef))
  (bind _currentlevel (Variables|/Game/Core/GameMode/GI_Base.GI_Base_C|GetCurrentLevel _gameinstanceref))
  (bind _result (Math|Integer|IncrementInt _currentlevel)
    (:%20%20
      (if (< _currentlevel 6)
        _
        (else
          (Development|PrintString "There should always be 5 levels. No more No less.")))
      (return _result))))

(fn SpawnDefaultPawnfor
  (params (NewPlayer :type Controller%20Object%20Reference) (StartSpot :type Actor%20Object%20Reference))
  (bind _asplayer_controller (Utilities|Casting|CastToPlayerController NewPlayer))
  (bind _asgi_base (Utilities|Casting|CastToGI_Base (Game|GetGameInstance)))
  (bind _isactive (Default|IsPlayerActive _asgi_base (Class|GameplayStatics|GetPlayerControllerID _asplayer_controller)))
  (if _isactive
    (bind _returnvalue (|CallParentFunction NewPlayer StartSpot))
    (return _returnvalue)
    (else
      (return 0))))