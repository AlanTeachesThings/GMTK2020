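; BP_HudBase is a HUD Blueprint that creates and shows the player's main HUD screen, with a TODO noting it is not yet co-op compatible.
; Its OpenHUD event creates WBP_HUDScreen for the owning player and adds it to the viewport.
; It passes the health bar to the BP_CharBase pawn and initializes the score widget with GM_Base, then focuses the game viewport.
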(event Custom|Open%20HUD
  ;[1 1 1] Setup and visualise HUDScreen. TODO: Make coop compatible
  (bind _returnvalue (UserInterface|CreateWidget "/Game/UI/HUD/WBP_HUDScreen.WBP_HUDScreen_C" (Variables|Default|GetPlayerOwner)))
  (UserInterface|Viewport|AddtoViewport _returnvalue 0)
  (bind _output_get (Variables|Default|SetHUD%20Screen _returnvalue))
  (bind _asbp_char_base (Utilities|Casting|CastToBP_CharBase (Class|HUD|GetOwningPawn)))
  (Default|SetupHealthUI _asbp_char_base (Variables|/Game/UI/HUD/WBP_HUDScreen.WBP_HUDScreen_C|GetWBP_HealthBar _output_get))
  (bind _asgm_base (Utilities|Casting|CastToGM_Base (Game|GetGameMode)))
  (Default|InitialSetup (Variables|/Game/UI/HUD/WBP_HUDScreen.WBP_HUDScreen_C|GetWBP_Score _output_get) _asgm_base)
  (Class|WidgetBlueprintLibrary|SetFocustoGameViewport))

(fn ConstructionScript)