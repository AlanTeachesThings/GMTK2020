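; BP_WeaponBase is a base weapon actor that snaps to its owner's WeaponSocket and fires projectiles for a BP_CharBase pawn.
; Trigger press fires immediately or after a cooldown delay and starts a looping timer, which trigger release clears; the logic is marked overridable.
; A multiplier scales fire rate and restarts active fire when updated.
; Projectiles receive velocity, damage and homing target, with Accuracy setting random cone spread around the pawn's aim.
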(event Custom|Fire
  ;[1 1 1] Fire Logic - Overidable
  (CallFunction|SpawnProjectile)
  (Variables|Runtime|SetLastFire (Utilities|Time|GetGameTimeinSeconds)))

(event Custom|Trigger%20Pressed
  ;[1 1 1] Fire Logic - Overidable
  (Variables|Runtime|SetTriggerIsPressed true)
  (if (> (+ (Variables|Runtime|GetLastFire) (CallFunction|GetFireRate)) (Utilities|Time|GetGameTimeinSeconds))
    (Utilities|FlowControl|Delay (CallFunction|GetFireRate))
    (if (Variables|Runtime|GetTriggerIsPressed)
      (CallFunction|SetTimer (CallFunction|GetFireRate) :!label _label)
      (CallFunction|Fire))
    (else
      (goto _label))))

(event Custom|Trigger%20Released
  ;[1 1 1] Fire Logic - Overidable
  (Variables|Runtime|SetTriggerIsPressed false)
  (Utilities|Time|ClearandInvalidateTimerbyHandle (Variables|Runtime|GetFire%20Timer)))

(event EventBeginPlay
  (CallFunction|SetupPawnandAttach))

(fn ConstructionScript)

(fn SpawnProjectile
  ;[1 1 1] Spawn Projectile at location
  (Game|SpawnActorfromClass (Variables|Weapon|GetProjectile) (CallFunction|CalculateProjSpawnTransform) "Undefined" self true (Variables|Weapon|GetVelocity) (Variables|Weapon|GetDamage) (Variables|Default|GetHoming%20Target) (Game|GetInstigator)))

(fn SetupPawnandAttach
  (bind _returnvalue (Components|GetOwner))
  (Transformation|AttachActorToActor _returnvalue "WeaponSocket" "SnapToTarget" "SnapToTarget" "KeepWorld" false)
  (bind _asbp_char_base (Utilities|Casting|CastToBP_CharBase _returnvalue))
  (Variables|Runtime|SetPawn%20Ref _asbp_char_base))

(fn GetFireRate
  (return (/ (Variables|Weapon|GetFire%20Rate) (Variables|Runtime|GetFire%20Rate%20Multiplier))))

(fn UpdateFireRate
  (params (Fire%20Rate%20Multi :type Float%20%28single-precision%29))
  (Variables|Runtime|SetFire%20Rate%20Multiplier Fire%20Rate%20Multi)
  (if (Utilities|Time|IsTimerActivebyHandle (Variables|Runtime|GetFire%20Timer))
    (CallFunction|TriggerPressed))
  (return))

(fn SetTimer
  (params (Time :type Float%20%28single-precision%29))
  (bind _returnvalue (Utilities|Time|SetTimerbyEvent (EventDispatchers|CreateEvent :!event Custom|Fire) Time true))
  (Variables|Runtime|SetFire%20Timer _returnvalue))

(fn CalculateProjSpawnTransform
  (return (Math|Transform|MakeTransform (Transformation|GetWorldLocation (Variables|Default|GetSceneRoot)) (Math|Conversions|RotationFromXVector (Math|Random|RandomUnitVectorinConeinDegrees (Variables|/Game/Core/BP_CharBase.BP_CharBase_C|GetAimDirection (Variables|Runtime|GetPawn%20Ref)) (Math|Float|MapRangeClamped (Variables|Weapon|GetAccuracy) 1e+02 0.0 0.0 9e+01))))))