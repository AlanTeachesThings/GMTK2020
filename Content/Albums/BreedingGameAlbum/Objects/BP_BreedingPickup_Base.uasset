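; Base pickup actor for the breeding game, collected by the player or by enemies and destroyed once picked up.
; On overlap, it accepts the player if pickup is allowed, or a breeding enemy that reports this pickup class as compatible.
; OnPickedUp is an empty hook for child classes to supply the effect.
; The construction script applies one Color to both the mesh material and the point light.
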(event Collision|EventActorBeginOverlap
  (params (OtherActor :type Actor%20Object%20Reference))
  ;[1 1 1] Check who is trying to pick up, and do pickups effect
  (bind _succeseful (CallFunction|CanActorPickThisUp OtherActor))
  (if _succeseful
    (CallFunction|OnPickedUp OtherActor)
    (Actor|DestroyActor)))

(fn ConstructionScript
  (bind _color (Variables|Default|GetColor))
  (Rendering|Material|SetVectorParameterValueonMaterials (Variables|Default|GetStaticMesh) "Color" (Math|Conversions|ToVector(LinearColor) _color))
  (Rendering|Components|Light|SetLightColor (Variables|Default|GetPointLight) _color true))

(fn HidePrimitives
  (Rendering|SetVisibility (Variables|Default|GetSphere) false true))

(fn OnPickedUp
  (params (ReceivingActor :type Actor%20Object%20Reference)))

(fn CanActorPickThisUp
  (params (HitActor :type Actor%20Object%20Reference))
  (Utilities|FlowControl|Sequence
    (:then_0
      (Utilities|Casting|CastToBP_PlayerChar HitActor)
      (if (Variables|Default|GetPlayerPickupAllowed)
        (return true)
        (else
          (return false))))
    (:then_1
      (bind _asbreeding_enemy_base_bp (Utilities|Casting|CastToBreeding_Enemy_Base_BP HitActor))
      (bind _compatible (Default|IsPickupCompatible _asbreeding_enemy_base_bp (Utilities|GetClass self)))
      (if _compatible
        (return true)
        (else
          (return false))))))