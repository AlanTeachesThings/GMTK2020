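; Player character Blueprint for the Breeding game album, layering weapon HUD and inventory setup onto its parent class.
; On BeginPlay it creates the current-weapon widget, shows the current weapon's name, conceals every inventory item, then selects the first weapon.
; The RotateMeshTowardsAim override passes a fixed interpolation speed to the parent, ignoring its input.
; A delayed HUD refresh is left unconnected, and Tick is disabled.
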(event EventBeginPlay
  (bind _inventory (Variables|Default|GetInventory))
  (|CallParentFunction)
  (bind _returnvalue (UserInterface|CreateWidget "/Game/Albums/BreedingGameAlbum/UI/WBP_CurrentWeapon.WBP_CurrentWeapon_C" (Game|GetPlayerController 0)))
  (bind _output_get (Variables|Default|SetCurrentWeaponWidget _returnvalue))
  (Default|UpdateWeaponHUD _output_get (Variables|/Game/Core/BP_WeaponBase.BP_WeaponBase_C|GetCleanWeaponName (Variables|Default|GetCurrent%20Weapon)))
  (UserInterface|Viewport|AddtoViewport _returnvalue 0)
  (for (_array_element _array_index) (Variables|/Game/Core/Components/Inventory.Inventory_C|GetInventory%20Runtime%20Object _inventory)
    (Default|ConcealInventoryItem _inventory _array_element _array_index))
  (CallFunction|SelectCurrentWeapon))

(event Collision|EventActorBeginOverlap
  (params (OtherActor :type Actor%20Object%20Reference)))

(event EventTick
  (params (DeltaSeconds :type Float%20%28single-precision%29))
  (|CallParentFunction DeltaSeconds) ; This node is disabled and will not be called.\nDrag off pins to build functionality.
)

(event Input|ActionEvents|InputActionCycleWeapons
  (params (Key :type Key%20Structure :default "None")))

(event Input|ActionEvents|InputActionWeaponSlot1
  (params (Key :type Key%20Structure :default "None")))

(event Input|ActionEvents|InputActionWeaponSlot2
  (params (Key :type Key%20Structure :default "None")))

(event Input|ActionEvents|InputActionWeaponSlot3
  (params (Key :type Key%20Structure :default "None")))

(fn ConstructionScript
  (|CallParentFunction))

(fn RotateMeshTowardsAim
  (params (InterpSpeed :type Float%20%28single-precision%29))
  (|CallParentFunction 15.0))