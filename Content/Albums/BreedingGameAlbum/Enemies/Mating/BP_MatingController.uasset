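; Mating controller for the breeding game that pairs breeders and spawns their offspring.
; RequestMate accepts class pairs found in DT_MatingLogic in either order, queueing timestamped requests until the partner makes a reciprocal one.
; A match spawns the child at the requesting breeder's transform from the queued request, broadcasts the spawn, and tells both parents whether they survive.
; Tick purges requests older than the validity duration.
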(event EventTick
  (params (DeltaSeconds :type Float%20%28single-precision%29))
  (CallFunction|RemoveOldRequests))

(fn ConstructionScript)

(fn RequestMate
  (params (RequestingBreeder :type Breeding%20Enemy%20Base%20BP%20Object%20Reference) (BreederToMateWith :type Breeding%20Enemy%20Base%20BP%20Object%20Reference))
  ;[1 1 1] Check Matching Logic
  (bind _matchinglogicexists (CallFunction|LookUpBreedResult (Utilities|Struct|MakeBreedRequest RequestingBreeder BreederToMateWith 0.0)))
  (if _matchinglogicexists
    ;[1 1 1] Check if Other breeder requested Mate as well
    (bind (_breedsuccesful _matchingrequest) (CallFunction|CheckifMatchExists RequestingBreeder BreederToMateWith))
    (if _breedsuccesful
      (CallFunction|Mate _matchingrequest)
      (else
        (Utilities|Array|Add (Variables|Default|GetRequestList) (Utilities|Struct|MakeBreedRequest RequestingBreeder BreederToMateWith (Utilities|Time|GetGameTimeinSeconds)))))))

(fn CheckifMatchExists
  (params (RequestingBreeder :type Breeding%20Enemy%20Base%20BP%20Object%20Reference) (BreederToMatchTo :type Breeding%20Enemy%20Base%20BP%20Object%20Reference))
  (for _array_element (Variables|Default|GetRequestList)
    (if (== BreederToMatchTo (.RequestingBreeder (Utilities|Struct|BreakBreedRequest _array_element))) ; Check if Match is in the requestlist
      (if (== (.BreederToMateWith (Utilities|Struct|BreakBreedRequest _array_element)) RequestingBreeder) ; Check if match is with requester
        (return true _array_element))))
  (return false ""))

(fn Mate
  (params (BreedRequest :type Breed%20Request%20Structure))
  (bind (_requestingbreeder _breedertomatewith) (Utilities|Struct|BreakBreedRequest BreedRequest))
  (bind (_matchinglogicexists _child _matessurvive) (CallFunction|LookUpBreedResult BreedRequest))
  (Utilities|FlowControl|Sequence
    (:then_0
      ;[1 1 1] Spawn Breeders
      (CallFunction|SpawnBreeder _child (Transformation|GetActorTransform (.RequestingBreeder (Utilities|Struct|BreakBreedRequest BreedRequest)))))
    (:then_1
      ;[1 1 1] CallBack to Breeders
      (Default|OnMateSuccess _requestingbreeder _matessurvive)
      (Default|OnMateSuccess _breedertomatewith _matessurvive))))

(fn LookUpBreedResult
  (params (BreedRequest :type Breed%20Request%20Structure))
  (bind (_requestingbreeder _breedertomatewith) (Utilities|Struct|BreakBreedRequest BreedRequest))
  ;[1 1 1] Set Local vars
  (LocalVariables|SetMate1 (Utilities|GetClass _requestingbreeder))
  (LocalVariables|SetMate2 (Utilities|GetClass _breedertomatewith))
  ;[1 1 1] Find MatingResult and return child
  (bind _outrownames (DataTable|GetDataTableRowNames "/Game/Albums/BreedingGameAlbum/Enemies/Mating/DT_MatingLogic.DT_MatingLogic"))
  (for _array_element _outrownames
    (bind _returnvalue (Utilities|GetDataTableRow "/Game/Albums/BreedingGameAlbum/Enemies/Mating/DT_MatingLogic.DT_MatingLogic" _array_element)
      (:then
        (if (.Match (Utilities|GetChildifMatching _returnvalue (LocalVariables|GetMate1) (LocalVariables|GetMate2)))
          (return true (.Child (Utilities|GetChildifMatching _returnvalue (LocalVariables|GetMate1) (LocalVariables|GetMate2))) (.MatesSurvive (Utilities|GetChildifMatching _returnvalue (LocalVariables|GetMate1) (LocalVariables|GetMate2))))
          (elif (.Match (Utilities|GetChildifMatching _returnvalue (LocalVariables|GetMate2) (LocalVariables|GetMate1)))
            (return true (.Child (Utilities|GetChildifMatching _returnvalue (LocalVariables|GetMate2) (LocalVariables|GetMate1))) (.MatesSurvive (Utilities|GetChildifMatching _returnvalue (LocalVariables|GetMate2) (LocalVariables|GetMate1)))))))))
  ;[1 1 1] Send message if no child is found.
  (return false 0 false) ; not found, return null
)

(fn SpawnBreeder
  (params (BreederToSpawn :type Breeding%20Enemy%20Base%20BP%20Class%20Reference) (SpawnLocation :type Transform))
  (bind _returnvalue (Game|SpawnActorfromClass BreederToSpawn SpawnLocation "AdjustIfPossibleButAlwaysSpawn" 0 0))
  (Default|CallOnBreederSpawned _returnvalue))

(fn RemoveOldRequests
  (for _array_element (Variables|Default|GetRequestList)
    ;[1 1 1] Remove requests that are no longer valid
    (if (< (+ (.RequestTimeStamp (Utilities|Struct|BreakBreedRequest _array_element)) (Variables|Default|GetRequestValidityDuration)) (Utilities|Time|GetGameTimeinSeconds))
      (Utilities|Array|RemoveItem (Variables|Default|GetRequestList) _array_element))))