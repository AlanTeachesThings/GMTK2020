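; Base enemy Blueprint for breeders in the breeding game that can mate, evolve and periodically drop items.
; On overlapping another breeder after its cooldown, it requests mating from the level's BP_MatingController, and it destroys itself if it does not survive.
; A looping timer spawns its drop class, either another breeder or a WallPiece.
; Evolve replaces it with a random class from EvolveInto, and movement toggles between walk and run speeds.
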(event Custom|OnMateSuccess
  (params (SurviveMating :type Boolean))
  (Variables|Default|SetBreedingTimer (Variables|Mating|GetBreedingCooldown))
  (if (not SurviveMating)
    (CallFunction|OnDestroy)))

(event Custom|OnLocationArrival
  (CallFunction|Walk))

(event Custom|Walk
  (bind _charactermovement (Variables|Character|GetCharacterMovement))
  ;[1 1 1] Set Movement speed to Walk or Run
  (if (not (Variables|Behaviour|GetisWalking))
    (Variables|Behaviour|SetisWalking true)
    (Variables|/Script/Engine.CharacterMovementComponent|SetMaxWalkSpeed _charactermovement (/ (Variables|/Script/Engine.CharacterMovementComponent|GetMaxWalkSpeed _charactermovement) (Variables|Behaviour|GetWalkMoveFactor)))))

(event Custom|Run
  (bind _charactermovement (Variables|Character|GetCharacterMovement))
  ;[1 1 1] Set Movement speed to Walk or Run
  (if (Variables|Behaviour|GetisWalking)
    (Variables|Behaviour|SetisWalking false)
    (Variables|/Script/Engine.CharacterMovementComponent|SetMaxWalkSpeed _charactermovement (* (Variables|/Script/Engine.CharacterMovementComponent|GetMaxWalkSpeed _charactermovement) (Variables|Behaviour|GetWalkMoveFactor)))))

(event EventBeginPlay
  ;[1 1 1] BeginPlay
  (|CallParentFunction)
  ;;[1 1 1] Get Mating Controller
  (bind _outactors (Actor|GetAllActorsOfClass "/Game/Albums/BreedingGameAlbum/Enemies/Mating/BP_MatingController.BP_MatingController_C"))
  (Variables|Default|SetMatingController (Utilities|Array|Get(acopy) _outactors))
  ;;[1 1 1] Start Dropping Items
  (if (Utilities|IsValidClass (Variables|ItemDrops|GetItemToDrop))
    (bind _returnvalue (Utilities|Time|SetTimerbyFunctionName self "DropItem" (Variables|ItemDrops|GetTimeBetweenItemDrops) true))
    (Variables|ItemDrops|SetItemDropTimerHandle _returnvalue)))

(event Collision|EventActorBeginOverlap
  (params (OtherActor :type Actor%20Object%20Reference))
  (bind (_asbreeding_enemy_base_bp _bsuccess) (Utilities|Casting|CastToBreeding_Enemy_Base_BP OtherActor))
  ;[1 1 1] Bumped into another Breeding Enemy - Request to Mate with them!
  (if _bsuccess
    (if (< (Variables|Default|GetBreedingTimer) 0.0)
      (Default|RequestMate (Variables|Default|GetMatingController) self _asbreeding_enemy_base_bp))))

(event EventTick
  (params (DeltaSeconds :type Float%20%28single-precision%29))
  ;[1 1 1] Breeding Timer to prevent constant breeding
  (|CallParentFunction DeltaSeconds)
  (Variables|Default|SetBreedingTimer (- (Variables|Default|GetBreedingTimer) DeltaSeconds)))

(fn ConstructionScript)

(fn IsPickupCompatible
  (params (PickupClass :type BP%20Breeding%20Pickup%20Base%20Class%20Reference))
  (return (Utilities|Array|ContainsItem (Variables|Default|GetCompatiblePickups) PickupClass)))

(fn DropItem
  (bind _itemtodrop (Variables|ItemDrops|GetItemToDrop))
  (if (Utilities|IsValidClass _itemtodrop)
    (bind _returnvalue (Game|SpawnActorfromClass _itemtodrop (Transformation|GetActorTransform self) "AdjustIfPossibleButAlwaysSpawn" 0 0))
    (bind _asbreeding_enemy_base_bp (Utilities|Casting|CastToBreeding_Enemy_Base_BP _returnvalue)
      (:then
        (Default|CallOnDropBreeder _asbreeding_enemy_base_bp))
      (:CastFailed
        ;[1 0 0.02893] TODO: Make this a generic call across objects
        (bind _aswall_piece (Utilities|Casting|CastToWallPiece _returnvalue))
        (Default|Pooped _aswall_piece)))))

(fn Evolve
  (bind _evolvedbreeder (CallFunction|GetEvolvedBreederClass))
  (if (Utilities|IsValidClass _evolvedbreeder)
    (bind _returnvalue (Game|SpawnActorfromClass _evolvedbreeder (Transformation|GetActorTransform self) "AdjustIfPossibleButAlwaysSpawn" 0 0))
    (Default|CallOnEvolve _returnvalue)
    (CallFunction|OnDestroy)))

(fn GetEvolvedBreederClass
  (bind _evolveinto (Variables|Default|GetEvolveInto))
  (if (>= (Utilities|Array|LastIndex (Variables|Default|GetEvolveInto)) 0)
    (Utilities|Array|Shuffle _evolveinto)
    (return (Utilities|Array|Get(acopy) _evolveinto))))