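; AI controller for enemies in the breeding game, extending a parent controller's behaviour tree initialisation.
; After the parent init, it seeds the blackboard with wander and fear settings read from the controlled Breeding_Enemy_Base_BP pawn.
; The pawn's WanderRadius feeds both the wander radius and maximum wander distance keys.
; The attract radius comes from AttractSphere class defaults rather than the pawn.
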(event EventBeginPlay
  (|CallParentFunction))

(event EventTick
  (params (DeltaSeconds :type Float%20%28single-precision%29)))

(fn ConstructionScript
  (|CallParentFunction))

(fn InitBehaviourTree
  (params (BTAsset :type Behavior%20Tree%20Object%20Reference) (Player%20Object%20Key :type Name :default "None"))
  (bind _self self)
  (bind _returnvalue (AI|GetBlackboard _self))
  (bind _returnvalue_2 (Pawn|GetControlledPawn _self))
  (bind _asbreeding_enemy_base_bp (Utilities|Casting|CastToBreeding_Enemy_Base_BP _returnvalue_2))
  (|CallParentFunction BTAsset Player%20Object%20Key)
  (AI|Components|Blackboard|SetValueasFloat _returnvalue (Utilities|Name|MakeLiteralName "WanderRadius") (Variables|/Game/Albums/BreedingGameAlbum/Enemies/Breeding_Enemy_Base_BP.Breeding_Enemy_Base_BP_C|GetWanderRadius _asbreeding_enemy_base_bp))
  (AI|Components|Blackboard|SetValueasFloat _returnvalue (Utilities|Name|MakeLiteralName "MaxWanderDistance") (Variables|/Game/Albums/BreedingGameAlbum/Enemies/Breeding_Enemy_Base_BP.Breeding_Enemy_Base_BP_C|GetWanderRadius _asbreeding_enemy_base_bp))
  (AI|Components|Blackboard|SetValueasFloat _returnvalue (Utilities|Name|MakeLiteralName "MinWanderDistance") (Variables|/Game/Albums/BreedingGameAlbum/Enemies/Breeding_Enemy_Base_BP.Breeding_Enemy_Base_BP_C|GetMinWanderRadius _asbreeding_enemy_base_bp))
  (AI|Components|Blackboard|SetValueasFloat _returnvalue (Utilities|Name|MakeLiteralName "FearRadius") (Variables|/Game/Albums/BreedingGameAlbum/Enemies/Breeding_Enemy_Base_BP.Breeding_Enemy_Base_BP_C|GetFearSenseRadius _asbreeding_enemy_base_bp))
  (AI|Components|Blackboard|SetValueasBool _returnvalue (Utilities|Name|MakeLiteralName "UseFearRadius") (Variables|/Game/Albums/BreedingGameAlbum/Enemies/Breeding_Enemy_Base_BP.Breeding_Enemy_Base_BP_C|GetUseFearRadius _asbreeding_enemy_base_bp))
  (AI|Components|Blackboard|SetValueasFloat _returnvalue (Utilities|Name|MakeLiteralName "AttractSphereRadius") (.AttractRadius (Utilities|GetClassDefaults "/Game/Albums/BreedingGameAlbum/GrenadeLauncher/AttractSphere.AttractSphere_C"))))