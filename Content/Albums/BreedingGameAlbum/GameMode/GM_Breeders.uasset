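; Game mode for the breeding game that tracks living breeders by color and judges each level's win condition.
; Breeders from spawners, the mating controller and level placement register through one function that binds their events.
; Spawns and deaths refresh the counter widget and compare the target color's count against the condition.
; A met condition runs a Tick countdown to end the level, and an empty population triggers a Grey wave.
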(event Custom|OnBreederSpawnedFromSpawner
  (params (Spawner :type BP%20AI%20Spawner%20Object%20Reference) (SpawnedEnemy :type BP%20Enemy%20Base%20Object%20Reference))
  ;[1 1 1] Bind to Spawner
  (bind _asbreeding_enemy_base_bp (Utilities|Casting|CastToBreeding_Enemy_Base_BP SpawnedEnemy))
  (CallFunction|OnBreederSpawned _asbreeding_enemy_base_bp))

(event Custom|OnBreederSpawnedFromMating
  (params (BreederSpawned :type Breeding%20Enemy%20Base%20BP%20Object%20Reference))
  ;[1 1 1] Bind to MatingController
  (CallFunction|OnBreederSpawned BreederSpawned))

(event EventStartNextLevel
  (bind _wincondition (Variables|Default|GetWinCondition))
  (bind (_breedertype _operator _targetcount) (Utilities|Struct|BreakWinCondition _wincondition))
  (|CallParentFunction)
  (bind _breeding_enemy (CallFunction|GetBreedingEnemyDisplayName _breedertype))
  (Default|SetTarget (Variables|Default|GetUICounterRef) _targetcount _operator _breeding_enemy)
  (Variables|Default|SetRemainingWinConditionTime (Variables|Default|GetWinConditionRequiredTime)))

(event EventBeginPlay
  (|CallParentFunction)
  (Utilities|FlowControl|Sequence
    (:then_0
      ;[1 1 1] Bind to Spawner
      (bind _outactors (Actor|GetAllActorsOfClass "/Game/Blueprints/Spawner/BP_AISpawner.BP_AISpawner_C"))
      (bind _output_get (Variables|Default|SetAISpawners _outactors))
      (for _array_element _output_get
        (EventDispatchers|BindEventtoOnAISpawned _array_element (delegate Custom|OnBreederSpawnedFromSpawner))))
    (:then_1
      ;[1 1 1] Bind to MatingController
      (bind _outactors_2 (Actor|GetAllActorsOfClass "/Game/Albums/BreedingGameAlbum/Enemies/Mating/BP_MatingController.BP_MatingController_C"))
      (bind _output_get_2 (Variables|Default|SetMatingController (Utilities|Array|Get(acopy) _outactors_2)))
      (EventDispatchers|BindEventtoOnBreederSpawned _output_get_2 (delegate Custom|OnBreederSpawnedFromMating)))
    (:then_2
      ;[1 1 1] Create UI
      (bind _returnvalue (UserInterface|CreateWidget "/Game/Albums/BreedingGameAlbum/UI/WBP_EnemyCounter.WBP_EnemyCounter_C" (Game|GetPlayerController 0)))
      (UserInterface|Viewport|AddtoViewport _returnvalue 0)
      (Variables|Default|SetUICounterRef _returnvalue))
    (:then_3
      ;[1 1 1] Get breeders already in level
      (bind _outactors_3 (Actor|GetAllActorsOfClass "/Game/Albums/BreedingGameAlbum/Enemies/Breeding_Enemy_Base_BP.Breeding_Enemy_Base_BP_C"))
      (for _array_element_2 _outactors_3
        (CallFunction|OnBreederSpawned _array_element_2)))))

(event EventTick
  (params (DeltaSeconds :type Float%20%28single-precision%29))
  (bind _uicounterref (Variables|Default|GetUICounterRef))
  (|CallParentFunction DeltaSeconds)
  ;[1 1 1] Update WinCondition Timer if WinCondition is Met
  (if (Variables|Default|GetWinConditionMet)
    (bind _output_get (Variables|Default|SetRemainingWinConditionTime (- (Variables|Default|GetRemainingWinConditionTime) DeltaSeconds)))
    (if (< _output_get 0.0)
      (Default|UpdateWinTimer _uicounterref false 0.0)
      (CallFunction|EndLevel)
      (else
        (Default|UpdateWinTimer _uicounterref true _output_get)))))

(event EventEndLevel
  (|CallParentFunction)
  (Variables|Default|SetWinConditionMet false))

(fn ConstructionScript
  (|CallParentFunction))

(fn OnBreederSpawned
  (params (Breeder%20spawned :type Breeding%20Enemy%20Base%20BP%20Object%20Reference))
  (Utilities|Array|Add (Variables|Default|GetBreedersAlive) Breeder%20spawned)
  (EventDispatchers|BindEventtoOnDeath Breeder%20spawned (EventDispatchers|CreateEvent :!event OnBreederDeath))
  (EventDispatchers|BindEventtoOnDropBreeder Breeder%20spawned (EventDispatchers|CreateEvent :!event OnBreederSpawned))
  (EventDispatchers|BindEventtoOnEvolve Breeder%20spawned (EventDispatchers|CreateEvent :!event OnBreederSpawned))
  (CallFunction|UpdateUI)
  (CallFunction|CheckWinCondition))

(fn OnBreederDeath
  (params (Character :type BP%20Char%20Base%20Object%20Reference))
  (bind _asbreeding_enemy_base_bp (Utilities|Casting|CastToBreeding_Enemy_Base_BP Character))
  (Utilities|Array|RemoveItem (Variables|Default|GetBreedersAlive) _asbreeding_enemy_base_bp)
  (CallFunction|UpdateUI)
  (CallFunction|CheckWinCondition))

(fn CheckWinCondition
  (bind _wincondition (Variables|Default|GetWinCondition))
  (bind (_breedertype _operator _targetcount) (Utilities|Struct|BreakWinCondition _wincondition))
  (Utilities|FlowControl|Sequence
    (:then_0
      (bind (_bluecount _greencount _redcount _purplecount _greycount) (CallFunction|CountBreeders))
      (bind _breeding_enemy (CallFunction|GetBreedingEnemyDisplayName _breedertype))
      (switch string _breeding_enemy
        (:Blue
          (LocalVariables|SetCount _bluecount))
        (:Green
          (LocalVariables|SetCount _greencount))
        (:Red
          (LocalVariables|SetCount _redcount))
        (:Purple
          (LocalVariables|SetCount _purplecount))
        (:Grey
          (LocalVariables|SetCount _greycount)))
      (bind _output_get (Variables|Default|SetWinConditionMet (Utilities|Select :Index _operator :NewEnumerator0 (== (LocalVariables|GetCount) _targetcount) :NewEnumerator1 (< (LocalVariables|GetCount) _targetcount) :NewEnumerator2 (> (LocalVariables|GetCount) _targetcount))))
      (Default|UpdateWinTimer (Variables|Default|GetUICounterRef) _output_get (Variables|Default|GetRemainingWinConditionTime))
      (if (not _output_get)
        (Variables|Default|SetRemainingWinConditionTime (Variables|Default|GetWinConditionRequiredTime))))
    (:then_1
      ;[1 1 1] Spawn extra enemies if all enemies are dead
      (if (== (Utilities|Array|Length (Variables|Default|GetBreedersAlive)) 0)
        (Default|SpawnWave (Utilities|Array|Get(acopy) (Variables|Default|GetAISpawners)) "/Game/Albums/BreedingGameAlbum/Enemies/Breeding_Enemy_Grey_BP.Breeding_Enemy_Grey_BP_C" 5 3.0)))))

(fn UpdateUI
  (bind (_bluecount _greencount _redcount _purplecount) (CallFunction|CountBreeders))
  (Default|SetValues (Variables|Default|GetUICounterRef) _bluecount _greencount _redcount _purplecount))

(fn CountBreeders
  (for _array_element (Variables|Default|GetBreedersAlive)
    (Utilities|Casting|CastToBreeding_Enemy_Blue_BP _array_element
      (:then
        (Math|Integer|IncrementInt (LocalVariables|GetBlue)))
      (:CastFailed
        (Utilities|Casting|CastToBreeding_Enemy_Green_BP _array_element
          (:then
            (Math|Integer|IncrementInt (LocalVariables|GetGreen)))
          (:CastFailed
            (Utilities|Casting|CastToBreeding_Enemy_Red_BP _array_element
              (:then
                (Math|Integer|IncrementInt (LocalVariables|GetRed)))
              (:CastFailed
                (Utilities|Casting|CastToBreeding_Enemy_Purple_BP _array_element
                  (:then
                    (Math|Integer|IncrementInt (LocalVariables|GetPurple)))
                  (:CastFailed
                    (Utilities|Casting|CastToBreeding_Enemy_Grey_BP _array_element)
                    (Math|Integer|IncrementInt (LocalVariables|GetGrey)))))))))))
  (return (LocalVariables|GetBlue) (LocalVariables|GetGreen) (LocalVariables|GetRed) (LocalVariables|GetPurple) (LocalVariables|GetGrey)))

(fn SetWinCondition
  (params (WinCondition :type Win%20Condition%20Structure))
  (Variables|Default|SetWinCondition WinCondition))